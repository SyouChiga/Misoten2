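; BP_Worker is a worker pawn that walks to an assigned Accident, resolves it, then returns to its Station to be destroyed.
; A state machine on Tick moves it forward facing its target, or calls Resolving with its work speed each frame while working.
; RandomWalk adds a periodically re-rolled yaw offset so the path wanders.
; Capsule overlaps detect arrival at the tagged accident collision or the Station, and a vanished Accident sends it home.
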(event `self.ReceiveTick`
  (params (DeltaSeconds :type "Float (single-precision)"))
  (bind (_returnvalue_roll _returnvalue_pitch _returnvalue_yaw) (`KismetMathLibrary.BreakRotator` (`KismetMathLibrary.FindLookAtRotation` (`self.K2_GetActorLocation`) (`self.K2_GetActorLocation` (`self.Station`)))))
  (bind (_returnvalue_roll_2 _returnvalue_pitch_2 _returnvalue_yaw_2) (`KismetMathLibrary.BreakRotator` (`KismetMathLibrary.FindLookAtRotation` (`self.K2_GetActorLocation`) (`self.K2_GetActorLocation` (`self.Accident`)))))
  (switch `/Game/MyGame/BluePrints/ENUM_WorkerState` (`self.State`)
    (:`NewEnumerator0`
      (`/Engine/EditorBlueprintResources/StandardMacros.IsValid` (`self.Accident`)
        (:`Is Valid`
          ;[1 1 1] 前進
          (`self.AddMovementInput` (`self.GetActorForwardVector`))
          ;[1 1 1] Accidentを向く
          (`self.K2_SetActorRotation` (`KismetMathLibrary.MakeRotator` 0.0 0.0 _returnvalue_yaw_2))
          (`self.RandomWalk`))
        (:`Is Not Valid`
          (set `self.State` "NewEnumerator2"))))
    (:`NewEnumerator1`
      ;[1 1 1] 解決中
      (`/Engine/EditorBlueprintResources/StandardMacros.IsValid` (`self.Accident`)
        (:`Is Valid`
          (`/Game/MyGame/BluePrints/BP_Accident.Resolving` (`self.Accident`) (`self.WorkSpeed`)))
        (:`Is Not Valid`
          (set `self.State` "NewEnumerator2"))))
    (:`NewEnumerator2`
      ;[1 1 1] 前進
      (`self.AddMovementInput` (`self.GetActorForwardVector`))
      ;[1 1 1] Stationを向く
      (`self.K2_SetActorRotation` (`KismetMathLibrary.MakeRotator` 0.0 0.0 _returnvalue_yaw))
      (`self.RandomWalk`))))

(event `self.CapsuleComponent.OnComponentBeginOverlap`
  (params (OverlappedComponent :type "PrimitiveComponent Object Reference") (OtherActor :type "Actor Object Reference") (OtherComp :type "PrimitiveComponent Object Reference") (OtherBodyIndex :type Integer) (bFromSweep :type Boolean) (SweepResult :type "HitResult Structure (by ref)"))
  (bind (_returnvalue_roll _returnvalue_pitch _returnvalue_yaw) (`KismetMathLibrary.BreakRotator` (`KismetMathLibrary.FindLookAtRotation` (`self.K2_GetActorLocation`) (`self.K2_GetActorLocation` OtherActor))))
  (switch `/Game/MyGame/BluePrints/ENUM_WorkerState` (`self.State`)
    (:`NewEnumerator0`
      ;[1 1 1] Accident到達
      (if (== (`self.Accident`) OtherActor)
        (if (`ActorComponent.ComponentHasTag` OtherComp "WorkerCollision")
          (`self.K2_SetActorRotation` (`KismetMathLibrary.MakeRotator` 0.0 0.0 _returnvalue_yaw))
          (set `self.State` "NewEnumerator1"))))
    (:`NewEnumerator2`
      ;[1 1 1] Station到達
      (if (== OtherActor (`self.Station`))
        (`/Game/MyGame/BluePrints/BP_Station.DestroyWorker` (`self.Station`) self)))))

(fn `RandomWalk`
  (set `self.RandomWalkDelay` (+ (`self.RandomWalkDelay`) (`GameplayStatics.GetWorldDeltaSeconds`)))
  (`self.K2_AddActorLocalRotation` (`KismetMathLibrary.MakeRotator` 0.0 0.0 (`self.RandomWalkDegree`)))
  (if (>= (`self.RandomWalkDelay`) (`self.RandomWalkDelayValue`))
    (set `self.RandomWalkDelay` 0.0)
    (set `self.RandomWalkDelayValue` (`KismetMathLibrary.RandomFloatInRange` (`self.RandomWalkTimeMin`) (`self.RandomWalkTimeMax`)))
    (bind _output_get (set `self.RandomWalkDegree` (`KismetMathLibrary.RandomFloatInRange` -20.0 20.0)))
    (`KismetSystemLibrary.PrintString` (`KismetStringLibrary.Conv_DoubleToString` _output_get))))

(fn `UserConstructionScript`)