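; Spline path actor that spawns Num BP_CurveCar actors evenly spaced along its length and serves as their route.
; Construction script flattens the spline by forcing every point's world Z and tangent Z to a constant.
; A DoOnce on Tick spawns the cars, passing itself and each one's starting distance.
; GetCurrentLocationAndRotation converts distance to world location, direction and rotation, optionally wrapping for loops and updating the car's stored distance.
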(event `self.ReceiveBeginPlay`)

(event `self.ReceiveTick`
  (params (DeltaSeconds :type "Float (single-precision)"))
  (`/Engine/EditorBlueprintResources/StandardMacros.DoOnce` false
    (:`Completed`
      (for _index (range (`self.Num`))
        (bind _returnvalue (* (/ (`KismetMathLibrary.Conv_IntToDouble` _index) (`KismetMathLibrary.Conv_IntToDouble` (`self.Num`))) (`SplineComponent.GetSplineLength` (`self.Spline`))))
        (bind _returnvalue_2 (`|SpawnActorFromClass` "/Game/MyGame/BluePrints/Car/BP_CurveCar.BP_CurveCar_C" (`KismetMathLibrary.MakeTransform` (`SplineComponent.GetLocationAtDistanceAlongSpline` (`self.Spline`) _returnvalue "Local") (`SplineComponent.GetRotationAtDistanceAlongSpline` (`self.Spline`) _returnvalue "Local")) "AlwaysSpawn" "OverrideRootScale" null self null))
        (set `/Game/MyGame/BluePrints/Car/BP_CurveCar.MoveLocalLength` _returnvalue _returnvalue_2)))))

(fn `GetCurrentLocationAndRotation`
  (params (Length :type "Float (double-precision)") (Loop :type Boolean) (CarRef :type "/Game/MyGame/BluePrints/Car/BP_CurveCar Object Reference"))
  (returns (Location :type "Vector Structure") (Direction :type "Vector Structure") (Rotation :type "Rotator Structure"))
  (locals (LocalLength :type "Float (double-precision)"))
  (bind _spline (`self.Spline`))
  (bind _locallength (`local.LocalLength`))
  (set `self.CarRef` CarRef)
  (if Loop
    (bind _output_get (set `local.LocalLength` (mod Length (`SplineComponent.GetSplineLength` (`self.Spline`)))))
    (else
      (set `local.LocalLength` Length)))
  (set `/Game/MyGame/BluePrints/Car/BP_CurveCar.MoveLocalLength` _output_get (`self.CarRef`))
  (return (`SplineComponent.GetLocationAtDistanceAlongSpline` _spline _locallength "World") (`SplineComponent.GetDirectionAtDistanceAlongSpline` _spline _locallength "World") (`SplineComponent.GetRotationAtDistanceAlongSpline` _spline _locallength "World")))

(fn `GetNumSplinePoint`
  (returns (ReturnValue :type Integer))
  (return (`SplineComponent.GetNumberOfSplinePoints` (`self.Spline`))))

(fn `UserConstructionScript`
  (`|ExecutionSequence`
    (:`then_0`
      ;[1 1 1] SplineのZ座標を0に固定
      (for _index (range (`SplineComponent.GetNumberOfSplinePoints` (`self.Spline`)))
        (bind (_returnvalue_x _returnvalue_y) (`KismetMathLibrary.BreakVector` (`SplineComponent.GetLocationAtSplinePoint` (`self.Spline`) _index "World")))
        (`SplineComponent.SetLocationAtSplinePoint` (`self.Spline`) _index (`KismetMathLibrary.MakeVector` _returnvalue_x _returnvalue_y 10.0) "World" true)
        (bind (_returnvalue_x_2 _returnvalue_y_2) (`KismetMathLibrary.BreakVector` (`SplineComponent.GetTangentAtSplinePoint` (`self.Spline`) _index "World")))
        (`SplineComponent.SetTangentAtSplinePoint` (`self.Spline`) _index (`KismetMathLibrary.MakeVector` _returnvalue_x_2 _returnvalue_y_2 10.0) "World" true)))))