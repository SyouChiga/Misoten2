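; BP_CarSignal is a traffic signal actor that cycles its SignalColor state from Blue to Yellow to Red and back to Blue.
; While IsUpdating is true, Tick switches on the current color and starts a Delay before advancing it, with yellow timed separately from blue and red.
; Each change only sets the variable and prints the new color.
; BeginPlay sets the Arrow component's mobility to Static.
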(event `self.ReceiveBeginPlay`
  (`SceneComponent.SetMobility` (`self.Arrow`) "Static"))

(event `self.ReceiveTick`
  (params (DeltaSeconds :type "Float (single-precision)"))
  (if (`self.IsUpdating`)
    (switch `/Game/MyGame/BluePrints/Car/ENUM_SignalColor` (`self.SignalColor`)
      (:`NewEnumerator0`
        (`KismetSystemLibrary.Delay` (`self.ChangeSignalColorTime`))
        (set `self.SignalColor` "NewEnumerator1")
        (`KismetSystemLibrary.PrintString` "Yellow"))
      (:`NewEnumerator1`
        (`KismetSystemLibrary.Delay` (`self.SignalYellowTime`))
        (set `self.SignalColor` "NewEnumerator2")
        (`KismetSystemLibrary.PrintString` "Red"))
      (:`NewEnumerator2`
        (`KismetSystemLibrary.Delay` (`self.ChangeSignalColorTime`))
        (set `self.SignalColor` "NewEnumerator0")
        (`KismetSystemLibrary.PrintString` "Blue")))))

(fn `UserConstructionScript`)