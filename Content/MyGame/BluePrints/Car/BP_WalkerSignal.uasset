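; BP_WalkerSignal is a pedestrian signal that cycles SignalColor from Blue to Yellow to Red and reports whether crossing is allowed.
; Tick switches on the current color into a Delay, using a shorter-named yellow time or the shared change time, then advances the color and resets Timer.
; Tick also accumulates Timer and sets CanCrossing while at least six seconds of ChangeSignalColorTime remain, regardless of color.
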(event `self.ReceiveTick`
  (params (DeltaSeconds :type "Float (single-precision)"))
  (`|ExecutionSequence`
    (:`then_0`
      (switch `/Game/MyGame/BluePrints/Car/ENUM_SignalColor` (`self.SignalColor`)
        (:`NewEnumerator0`
          (`KismetSystemLibrary.Delay` (`self.ChangeSignalColorTime`))
          (set `self.SignalColor` "NewEnumerator1")
          (set `self.Timer` 0.0))
        (:`NewEnumerator1`
          (`KismetSystemLibrary.Delay` (`self.SignalYellowTime`))
          (set `self.SignalColor` "NewEnumerator2")
          (set `self.Timer` 0.0))
        (:`NewEnumerator2`
          (`KismetSystemLibrary.Delay` (`self.ChangeSignalColorTime`))
          (set `self.SignalColor` "NewEnumerator0")
          (set `self.Timer` 0.0))))
    (:`then_1`
      (set `self.Timer` (+ (`self.Timer`) DeltaSeconds))
      (if (>= (- (`self.ChangeSignalColorTime`) (`self.Timer`)) 6.0)
        (set `self.CanCrossing` true)
        (else
          (set `self.CanCrossing` false))))))

(fn `UserConstructionScript`
  (`parent.UserConstructionScript`))