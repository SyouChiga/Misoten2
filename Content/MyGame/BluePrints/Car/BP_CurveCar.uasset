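; BP_CurveCar is a car actor that drives itself in a loop along a spline, stopping for signals and other cars.
; Box overlaps record the current BP_CarSignal and contact with another BP_CurveCar.
; Tick brakes for that contact, or when the signal's arrow opposes the car and its brake area contains a BP_Car.
; Speed switches instantly between zero and cruising, advancing the spline distance that sets location (swept) and rotation.
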(event `self.ReceiveBeginPlay`
  (`/Engine/EditorBlueprintResources/StandardMacros.IsValid` (`self.UsingSpline`)))

(event `self.ReceiveTick`
  (params (DeltaSeconds :type "Float (single-precision)"))
  (`|ExecutionSequence`
    (:`then_0`
      ;[1 1 1] Overlapちゅうの信号があるとき
      (if (`KismetSystemLibrary.IsValid` (`self.OverlappingSignal`))
        (`KismetSystemLibrary.PrintString` "OverlappingSignalCollision")
        (if (< (`KismetMathLibrary.Dot_VectorVector` (`SceneComponent.GetForwardVector` (`/Game/MyGame/BluePrints/Car/Signals/BP_CarSignal.Arrow` (`self.OverlappingSignal`))) (`self.GetActorForwardVector`)) 0.0)
          (if (> (`KismetArrayLibrary.Array_Length` (`PrimitiveComponent.GetOverlappingActors` (`/Game/MyGame/BluePrints/Car/Signals/BP_CarSignal.BrakeAreaCollision` (`self.OverlappingSignal`)) "/Game/MyGame/BluePrints/Car/BP_Car.BP_Car_C")) 0)
            (set `self.IsBraking` true)
            (else
              (if (`self.IsHittingCar`) :!label _label
                (set `self.IsBraking` true)
                (else
                  (set `self.IsBraking` false))))))
        (else
          (goto _label))))
    (:`then_1`
      (if (`self.IsBraking`)
        (set `self.Speed` 0.0)
        (else
          (set `self.Speed` 750.0))))
    (:`then_2`
      ;[1 1 1] Spline上をMoveTime*Speed分移動させる　ついでに回転なども行う
      (set `self.MoveLocalLength` (+ (`self.MoveLocalLength`) (* (`GameplayStatics.GetWorldDeltaSeconds`) (`self.Speed`))))
      (bind (_location _direction _rotation) (`/Game/MyGame/BluePrints/Car/BP_CurveCarSpline.GetCurrentLocationAndRotation` (`self.UsingSpline`) (`self.MoveLocalLength`) true self))
      (`self.K2_SetActorLocation` _location true)
      (`self.K2_SetActorRotation` _rotation)
      (`KismetSystemLibrary.PrintString` (`KismetStringLibrary.Conv_DoubleToString` (`self.Speed`))))))

(event `self.Box.OnComponentBeginOverlap`
  (params (OverlappedComponent :type "PrimitiveComponent Object Reference") (OtherActor :type "Actor Object Reference") (OtherComp :type "PrimitiveComponent Object Reference") (OtherBodyIndex :type Integer) (bFromSweep :type Boolean) (SweepResult :type "HitResult Structure (by ref)"))
  ;[1 1 1] 信号か車にOverlapしているかを判断
  (`|ExecutionSequence`
    (:`then_0`
      (bind _asbp_car_signal (cast `/Game/MyGame/BluePrints/Car/Signals/BP_CarSignal` OtherActor))
      (set `self.OverlappingSignal` _asbp_car_signal)
      (`KismetSystemLibrary.PrintString` "Hello"))
    (:`then_1`
      (bind _asbp_curve_car (cast `/Game/MyGame/BluePrints/Car/BP_CurveCar` OtherActor))
      (if (!= _asbp_curve_car self)
        (set `self.IsHittingCar` true)))))

(event `self.Box.OnComponentEndOverlap`
  (params (OverlappedComponent :type "PrimitiveComponent Object Reference") (OtherActor :type "Actor Object Reference") (OtherComp :type "PrimitiveComponent Object Reference") (OtherBodyIndex :type Integer))
  ;[1 1 1] 信号か車にOverlapしているかを判断
  (`|ExecutionSequence`
    (:`then_0`
      (cast `/Game/MyGame/BluePrints/Car/Signals/BP_CarSignal` OtherActor)
      (set `self.OverlappingSignal` (`self.NullSignalRef`)))
    (:`then_1`
      (cast `/Game/MyGame/BluePrints/Car/BP_CurveCar` OtherActor)
      (set `self.IsHittingCar` false))))

(fn `UserConstructionScript`)