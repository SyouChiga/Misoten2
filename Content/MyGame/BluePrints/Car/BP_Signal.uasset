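; BP_Signal is a traffic signal in the Car folder that cycles its SignalColor state from Blue to Yellow to Red.
; Tick switches on the state and uses a latent Delay before each change, with Yellow timed separately from Blue and Red.
; Tick also prints the current color every frame as debug output.
; The construction script shows or hides two cube components from IsSignalVisible; the color never drives any visuals here.
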(event `self.ReceiveBeginPlay`)

(event `self.ReceiveTick`
  (params (DeltaSeconds :type "Float (single-precision)"))
  (bind _signalcolor (`self.SignalColor`))
  (`|ExecutionSequence`
    (:`then_0`
      (switch `/Game/MyGame/BluePrints/Car/ENUM_SignalColor` _signalcolor
        (:`NewEnumerator0`
          (`KismetSystemLibrary.Delay` (`self.ChangeSignalColorTime`))
          (set `self.SignalColor` "NewEnumerator1"))
        (:`NewEnumerator1`
          (`KismetSystemLibrary.Delay` (`self.SignalYellowTime`))
          (set `self.SignalColor` "NewEnumerator2"))
        (:`NewEnumerator2`
          (`KismetSystemLibrary.Delay` (`self.ChangeSignalColorTime`))
          (set `self.SignalColor` "NewEnumerator0"))))
    (:`then_1`
      (`KismetSystemLibrary.PrintString` (`|GetEnumeratorNameAsString` _signalcolor)))))

(fn `UserConstructionScript`
  (`SceneComponent.SetVisibility` (`self.Cube`) (`self.IsSignalVisible`) false)
  (`SceneComponent.SetVisibility` (`self.Cube1`) (`self.IsSignalVisible`) false))