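; BP_WalkerSignal is a pedestrian crossing signal that cycles Blue, Yellow and Red and exposes whether walkers can cross.
; While IsUpdating is set, Tick switches on SignalColor and uses Delays to advance it after configurable durations.
; Tick also accumulates Timer and sets CanCross only during Blue with at least three seconds of ChangeSignalColorTime remaining by that Timer.
; The Timer reset is unconnected, so the count carries across phases.
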(event `self.ReceiveTick`
  (params (DeltaSeconds :type "Float (single-precision)"))
  (if (`self.IsUpdating`)
    (`|ExecutionSequence`
      (:`then_0`
        (switch `/Game/MyGame/BluePrints/Car/ENUM_SignalColor` (`self.SignalColor`)
          (:`NewEnumerator0`
            (`KismetSystemLibrary.Delay` (`self.ChangeSignalColorTime`))
            (set `self.SignalColor` "NewEnumerator1"))
          (:`NewEnumerator1`
            (`KismetSystemLibrary.Delay` (`self.SignalYellowTime`))
            (set `self.SignalColor` "NewEnumerator2"))
          (:`NewEnumerator2`
            (`KismetSystemLibrary.Delay` (`self.ChangeSignalColorTime`))
            (set `self.SignalColor` "NewEnumerator0"))))
      (:`then_1`
        (bind _output_get (set `self.Timer` (+ DeltaSeconds (`self.Timer`))))
        (set `self.CanCross` false)
        (if (and (`|EnumEquality` (`self.SignalColor`) "NewEnumerator0") (>= (- (`self.ChangeSignalColorTime`) _output_get) 3.0))
          (set `self.CanCross` true)
          (else
            (set `self.CanCross` false)))))))

(fn `UserConstructionScript`)