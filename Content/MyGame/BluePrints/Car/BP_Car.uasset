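; BP_Car is an AI traffic car that loops along a spline, braking for obstacles and signals.
; Each tick it brakes for pedestrians in its Box, cars hit by a forward trace, or yellow and red BP_CarSignals facing against it, checked by dot product.
; The brake flag ramps Speed down or up within limits.
; Speed advances a distance along UsingSpline, which supplies location and rotation; SetLength can override that distance.
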(event `self.ReceiveBeginPlay`
  ;[1 1 1] Splineからの距離を計算し、Speedで割って出た時間をMoveTimeにする
  (set `self.MoveLocalLength` (`KismetMathLibrary.VSize` (- (`self.K2_GetActorLocation`) (`self.K2_GetActorLocation` (`self.UsingSpline`))))))

(event `self.ReceiveTick`
  (params (DeltaSeconds :type "Float (single-precision)"))
  (bind _frontarrow (`self.FrontArrow`))
  (bind _overlappingactors (`PrimitiveComponent.GetOverlappingActors` (`self.Box1`) "/Game/MyGame/BluePrints/Car/Signals/BP_CarSignal.BP_CarSignal_C"))
  (bind _returnvalue (`SceneComponent.K2_GetComponentLocation` _frontarrow))
  (bind _asbp_car_signal (cast `/Game/MyGame/BluePrints/Car/Signals/BP_CarSignal` (`|GetArrayItem` _overlappingactors) :!pure true))
  (`|ExecutionSequence`
    (:`then_0`
      ;[1 1 1] 歩行者が前にいた場合、止まる
      (if (> (`KismetArrayLibrary.Array_Length` (`PrimitiveComponent.GetOverlappingActors` (`self.Box`) "/Game/MyGame/BluePrints/AI/BP_Walker.BP_Walker_C")) 0)
        (set `self.IsBraking` true)
        (else
          (`|ExecutionSequence`
            (:`then_0`
              ;[1 1 1] 前方向にRayをとばして車と当たってたらブレーキ
              (bind _outhit (`KismetSystemLibrary.LineTraceSingle` _returnvalue (+ _returnvalue (* (`SceneComponent.GetForwardVector` _frontarrow) 500.0)) "TraceTypeQuery1"))
              (cast `/Game/MyGame/BluePrints/Car/BP_Car` (`.HitActor` (`GameplayStatics.BreakHitResult` _outhit))
                (:`then`
                  (set `self.IsBraking` true))
                (:`CastFailed`
                  (set `self.IsBraking` false))))))))
    (:`then_1`
      (if (> (`KismetArrayLibrary.Array_Length` _overlappingactors) 0)
        (if (`KismetMathLibrary.InRange_FloatFloat` (`KismetMathLibrary.Dot_VectorVector` (`SceneComponent.GetForwardVector` (`/Game/MyGame/BluePrints/Car/Signals/BP_CarSignal.Arrow` _asbp_car_signal)) (`SceneComponent.GetForwardVector` (`self.FrontArrow`))) -1.0 -0.7)
          (switch `/Game/MyGame/BluePrints/Car/ENUM_SignalColor` (`/Game/MyGame/BluePrints/Car/Signals/BP_CarSignal.SignalColor` _asbp_car_signal)
            (:`NewEnumerator1`
              _)
            (:`NewEnumerator2`
              _))
          (set `self.IsBraking` true))))
    (:`then_2`
      ;[1 1 1] アクセルとブレーキの処理
      (if (`self.IsBraking`)
        (set `self.Speed` (`KismetMathLibrary.FMax` (- (`self.Speed`) (`self.BreakePower`)) 1.0))
        (else
          (set `self.Speed` (`KismetMathLibrary.FMin` (+ (`self.Speed`) (`self.AccelPower`)) 750.0)))))
    (:`then_3`
      ;[1 1 1] Spline上をMoveTime*Speed分移動させる　ついでに回転なども行う
      (bind _output_get (set `self.MoveLocalLength` (+ (`self.MoveLocalLength`) (* (`GameplayStatics.GetWorldDeltaSeconds`) (`self.Speed`)))))
      (bind (_location _direction _rotation) (`/Game/MyGame/BluePrints/Car/BP_CarSpline.GetCurrentLocationAndRotation` (`self.UsingSpline`) _output_get true self))
      (`self.K2_SetActorLocation` (`KismetMathLibrary.MakeVector` (.x _location) (.y _location) (.z _location)) true)
      (`self.K2_SetActorRotation` _rotation))))

(fn `SetLength`
  (params (NewLength :type "Float (double-precision)"))
  (set `self.MoveLocalLength` NewLength))

(fn `UserConstructionScript`)