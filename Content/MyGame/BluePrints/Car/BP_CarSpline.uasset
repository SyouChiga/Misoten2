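; BP_CarSpline is a spline path actor that spawns cars and serves as the route reference they receive.
; On BeginPlay it spawns a set number of BP_Car actors at random XY positions, passing itself as their spline.
; The construction script flattens the spline by forcing every point's world Z and tangent Z to 1.
; Helper functions return point count and location, direction and rotation at a distance, with optional loop wrapping.
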(event `self.ReceiveBeginPlay`
  (for _ (range (`self.SpawnValueCar`))
    (`|SpawnActorFromClass` "/Game/MyGame/BluePrints/Car/BP_Car.BP_Car_C" (`KismetMathLibrary.MakeTransform` (`KismetMathLibrary.MakeVector` (`KismetMathLibrary.RandomFloatInRange` (* (`self.RandomSpawnMaxLength`) -1.0) (`self.RandomSpawnMaxLength`)) (`KismetMathLibrary.RandomFloatInRange` (* (`self.RandomSpawnMaxLength`) -1.0) (`self.RandomSpawnMaxLength`)))) "AlwaysSpawn" "OverrideRootScale" null self null)))

(fn `GetCurrentLocationAndRotation`
  (params (Length :type "Float (double-precision)") (Loop :type Boolean))
  (returns (Location :type "Vector Structure") (Direction :type "Vector Structure") (Rotation :type "Rotator Structure"))
  (locals (LocalLength :type "Float (double-precision)"))
  (bind _spline (`self.Spline`))
  (bind _locallength (`local.LocalLength`))
  (if Loop
    (set `local.LocalLength` (mod Length (`SplineComponent.GetSplineLength` (`self.Spline`))))
    (else
      (set `local.LocalLength` Length)))
  (return (`SplineComponent.GetLocationAtDistanceAlongSpline` _spline _locallength "World") (`SplineComponent.GetDirectionAtDistanceAlongSpline` _spline _locallength "World") (`SplineComponent.GetRotationAtDistanceAlongSpline` _spline _locallength "World")))

(fn `GetNumSplinePoint`
  (returns (ReturnValue :type Integer))
  (return (`SplineComponent.GetNumberOfSplinePoints` (`self.Spline`))))

(fn `UserConstructionScript`
  (`KismetSystemLibrary.PrintString` (`KismetStringLibrary.Conv_DoubleToString` (`SplineComponent.GetSplineLength` (`self.Spline`))))
  ;[1 1 1] SplineのZ座標を0に固定
  (for _index (range (`SplineComponent.GetNumberOfSplinePoints` (`self.Spline`)))
    (bind (_returnvalue_x _returnvalue_y) (`KismetMathLibrary.BreakVector` (`SplineComponent.GetLocationAtSplinePoint` (`self.Spline`) _index "World")))
    (`SplineComponent.SetLocationAtSplinePoint` (`self.Spline`) _index (`KismetMathLibrary.MakeVector` _returnvalue_x _returnvalue_y 1.0) "World" true)
    (bind (_returnvalue_x_2 _returnvalue_y_2) (`KismetMathLibrary.BreakVector` (`SplineComponent.GetTangentAtSplinePoint` (`self.Spline`) _index "World")))
    (`SplineComponent.SetTangentAtSplinePoint` (`self.Spline`) _index (`KismetMathLibrary.MakeVector` _returnvalue_x_2 _returnvalue_y_2 1.0) "World" true)))