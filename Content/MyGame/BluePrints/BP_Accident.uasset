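; BP_Accident is an accident actor that stays in the world until enough work has resolved it.
; On BeginPlay it stores the farthest BP_Walker inside WalkerCollision as MostFarWalker, and later overlaps fill that reference only while it is invalid.
; Resolving adds work speed scaled by delta time to Resolution.
; Tick checks that progress against ResolutionValue and asks AccidentGenerator to destroy the accident once reached.
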(event `self.ReceiveBeginPlay`
  (bind _returnvalue (`self.K2_GetActorLocation`))
  (bind _mostfarwalker (`self.MostFarWalker`))
  (bind _overlappingactors (`PrimitiveComponent.GetOverlappingActors` (`self.WalkerCollision`) "/Game/MyGame/BluePrints/BP_Walker.BP_Walker_C"))
  ;[1 1 1] 生成時最遠通行人算出
  (if (> (`KismetArrayLibrary.Array_Length` _overlappingactors) 0)
    (for _array_element _overlappingactors
      (`/Engine/EditorBlueprintResources/StandardMacros.IsValid` _mostfarwalker
        (:`Is Valid`
          (if (>= (`KismetMathLibrary.VSizeSquared` (- (`self.K2_GetActorLocation` _array_element) _returnvalue)) (`KismetMathLibrary.VSizeSquared` (- _returnvalue (`self.K2_GetActorLocation` _mostfarwalker))))
            (bind _asbp_walker (cast `/Game/MyGame/BluePrints/BP_Walker` _array_element :!label _label))
            (set `self.MostFarWalker` _asbp_walker)))
        (:`Is Not Valid`
          (goto _label))))))

(event `self.ReceiveTick`
  (params (DeltaSeconds :type "Float (single-precision)"))
  ;[1 1 1] Accident解決チェック
  (bind _isfinish (`self.CheckIsFinish`))
  (if _isfinish
    (`/Game/MyGame/BluePrints/BP_AccidentGenerator.DestroyAccident` (`self.AccidentGenerator`) self)))

(event `self.WalkerCollision.OnComponentBeginOverlap`
  (params (OverlappedComponent :type "PrimitiveComponent Object Reference") (OtherActor :type "Actor Object Reference") (OtherComp :type "PrimitiveComponent Object Reference") (OtherBodyIndex :type Integer) (bFromSweep :type Boolean) (SweepResult :type "HitResult Structure (by ref)"))
  ;[1 1 1] 最遠通行人
  (`/Engine/EditorBlueprintResources/StandardMacros.IsValid` (`self.MostFarWalker`)
    (:`Is Not Valid`
      (bind _asbp_walker (cast `/Game/MyGame/BluePrints/BP_Walker` OtherActor))
      (set `self.MostFarWalker` _asbp_walker))))

(fn `CheckIsFinish`
  (returns (IsFinish :type Boolean))
  (return (>= (`self.Resolution`) (`self.ResolutionValue`))))

(fn `Resolving`
  (params (WorkSpeed :type "Float (double-precision)"))
  (set `self.Resolution` (+ (* WorkSpeed (`GameplayStatics.GetWorldDeltaSeconds`)) (`self.Resolution`)))
  (return))

(fn `UserConstructionScript`)