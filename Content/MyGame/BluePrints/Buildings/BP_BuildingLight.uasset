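; Building light actor that wraps a rect light whose emitting area follows the actor's scale.
; The construction script maps Y scale to source width and Z scale to source height at 100 units per scale unit, then applies the Intensity variable to the light.
; It has no active runtime logic, as the event graph holds only disabled placeholder events.
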(fn `UserConstructionScript`
  (bind (_returnvalue_x _returnvalue_y) (`KismetMathLibrary.BreakVector` (`self.GetActorScale3D`)))
  (bind (_returnvalue_x_2 _returnvalue_y_2 _returnvalue_z) (`KismetMathLibrary.BreakVector` (`self.GetActorScale3D`)))
  (`RectLightComponent.SetSourceWidth` (`self.RectLight`) (* _returnvalue_y 100.0))
  (`RectLightComponent.SetSourceHeight` (`self.RectLight`) (* _returnvalue_z 100.0))
  (`LightComponent.SetIntensity` (`self.RectLight`) (`self.Intensity`)))