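; BP_PoliceStation is a police station that spawns BP_Police workers for accidents, up to a worker limit.
; SpawnWorker creates an officer at the given location, passing it the accident and the station itself, then adds it to the Workers array.
; It returns whether a spawn was allowed, refusing once the array reaches WorkerLimit.
; The event graph and construction script add no logic of their own.
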(fn `SpawnWorker`
  (params (Accident :type "/Game/MyGame/BluePrints/Accident/BP_Accident Object Reference") (SpawnLocation :type "Vector Structure"))
  (returns (IsSuccess :type Boolean))
  (if (> (`self.WorkerLimit`) (`KismetArrayLibrary.Array_Length` (`self.Workers`)))
    (bind _returnvalue (`|SpawnActorFromClass` "/Game/MyGame/BluePrints/Worker/Police/BP_Police.BP_Police_C" (`KismetMathLibrary.MakeTransform` SpawnLocation) "Undefined" "OverrideRootScale" null Accident self null))
    (`KismetArrayLibrary.Array_Add` (`self.Workers`) _returnvalue)
    (return true)
    (else
      (return false))))

(fn `UserConstructionScript`
  (`parent.UserConstructionScript`))