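; BP_WalkerNotCrowd is a walker actor that replaces itself with a BP_WalkerCrowd AI when the player comes within CrowdChangeLength.
; On its first Tick it caches the first BP_Player found, then compares squared distance to the player every Tick.
; Within range, it spawns BP_WalkerCrowd with BT_WalkerCrowd at its mesh's location and rotation, calls SpawnDefaultController on the new pawn, and destroys itself.
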(event `self.ReceiveTick`
  (params (DeltaSeconds :type "Float (single-precision)"))
  (bind (_returnvalue_location _returnvalue_rotation) (`KismetMathLibrary.BreakTransform` (`SceneComponent.K2_GetComponentToWorld` (`self.Mesh`))))
  (`parent.ReceiveTick` DeltaSeconds)
  (`/Engine/EditorBlueprintResources/StandardMacros.IsValid` self
    (:`Is Valid`
      (`|ExecutionSequence`
        (:`then_0`
          (`/Engine/EditorBlueprintResources/StandardMacros.DoOnce` false
            (:`Completed`
              ;[1 1 1] Player取得
              (bind _outactors (`GameplayStatics.GetAllActorsOfClass` "/Game/MyGame/BluePrints/Player/BP_Player.BP_Player_C"))
              (set `self.Player` (`|GetArrayItem` _outactors)))))
        (:`then_1`
          ;[1 1 1] Playerとの距離を見て一定以下だった場合、Crowdをスポーンし、自分を破棄
          (if (< (`KismetMathLibrary.VSizeSquared` (- (`self.K2_GetActorLocation` (`self.Player`)) (`self.K2_GetActorLocation`))) (`KismetMathLibrary.Square` (`self.CrowdChangeLength`)))
            (bind _returnvalue (`AIBlueprintHelperLibrary.SpawnAIFromClass` "/Game/MyGame/BluePrints/AI/BP_WalkerCrowd.BP_WalkerCrowd_C" "/Game/MyGame/BluePrints/AI/BehaviorTree/BT_WalkerCrowd.BT_WalkerCrowd" _returnvalue_location _returnvalue_rotation))
            (`/Engine/EditorBlueprintResources/StandardMacros.IsValid` _returnvalue
              (:`Is Valid`
                (`self.SpawnDefaultController` _returnvalue))
              (:`Is Not Valid`
                _))
            (`self.K2_DestroyActor`)))))))

(fn `UserConstructionScript`
  (`parent.UserConstructionScript`))