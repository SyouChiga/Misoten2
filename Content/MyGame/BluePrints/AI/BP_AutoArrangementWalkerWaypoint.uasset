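; Populates a twelve-segment circular map at BeginPlay by copying one hand-placed segment of waypoints, area collisions, walkers, intersections, car splines and car-update areas around it.
; Existing actors of each type are attached to per-type container components, then the actor rotates in 30-degree yaw steps, spawning copies at the children's world transforms.
; Intersection copies get fixed height and scale.
; After the full turn, the containers detach, keeping world transforms.
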(event `self.ReceiveBeginPlay`
  (bind (_returnvalue_roll _returnvalue_pitch _returnvalue_yaw) (`KismetMathLibrary.BreakRotator` (`self.K2_GetActorRotation`)))
  (`|ExecutionSequence`
    (:`then_0`
      ;[1 1 1] WayPointを検出してWaypoints子コンポーネントとしてアタッチする
      (bind _outactors (`GameplayStatics.GetAllActorsOfClass` "/Game/MyGame/BluePrints/AI/BP_WayPoint.BP_WayPoint_C"))
      (for _array_element _outactors
        (`self.K2_AttachToComponent` _array_element (`self.WayPoints`) "None" "KeepRelative" "KeepRelative" "KeepRelative" true))
      ;[1 1 1] AreaCollisionを検出してAreaCollisionsの子コンポーネントとしてアタッチする
      (bind _outactors_2 (`GameplayStatics.GetAllActorsOfClass` "/Game/MyGame/BluePrints/AI/BP_AreaCollision.BP_AreaCollision_C"))
      (for _array_element_2 _outactors_2
        (`self.K2_AttachToComponent` _array_element_2 (`self.AreaCollisions`) "None" "KeepRelative" "KeepRelative" "KeepRelative" true))
      ;[1 1 1] walkerNotCrowdを検出してWalkersに子コンポーネントとしてアタッチする
      (bind _outactors_3 (`GameplayStatics.GetAllActorsOfClass` "/Game/MyGame/BluePrints/AI/BP_WalkerNotCrowd.BP_WalkerNotCrowd_C"))
      (for _array_element_3 _outactors_3
        (`self.K2_AttachToComponent` _array_element_3 (`self.Walkers`) "None" "KeepRelative" "KeepRelative" "KeepRelative" true))
      (bind _outactors_4 (`GameplayStatics.GetAllActorsOfClass` "/Game/MyGame/BluePrints/Car/BP_InterSection.BP_InterSection_C"))
      (for _array_element_4 _outactors_4
        (`self.K2_AttachToComponent` _array_element_4 (`self.Signals`) "None" "KeepRelative" "KeepRelative" "KeepRelative" true))
      (bind _outactors_5 (`GameplayStatics.GetAllActorsOfClass` "/Game/MyGame/BluePrints/Car/BP_CarSpline.BP_CarSpline_C"))
      (for _array_element_5 _outactors_5
        (`self.K2_AttachToComponent` _array_element_5 (`self.Cars`) "None" "KeepRelative" "KeepRelative" "KeepRelative" true))
      (bind _outactors_6 (`GameplayStatics.GetAllActorsOfClass` "/Game/MyGame/BluePrints/Car/BP_UpdateCarArea.BP_UpdateCarArea_C"))
      (for _array_element_6 _outactors_6
        (`self.K2_AttachToComponent` _array_element_6 (`self.UpdateCarCollisions`) "None" "KeepRelative" "KeepRelative" "KeepRelative" true)))
    (:`then_1`
      ;[0.5426 0.5431 1] Map12分割なので30度ずつずらす
      (for _index (range 12)
        (`self.K2_SetActorRotation` (`KismetMathLibrary.MakeRotator` 0.0 0.0 (+ _returnvalue_yaw 30.0)))
        (if (not (== _index 11))
          ;;[1 1 1] WayPointを配置
          (for _array_element_7 (`SceneComponent.GetChildrenComponents` (`self.WayPoints`) false)
            (`|SpawnActorFromClass` "/Game/MyGame/BluePrints/AI/BP_WayPoint.BP_WayPoint_C" (`SceneComponent.K2_GetComponentToWorld` _array_element_7) "AlwaysSpawn" "OverrideRootScale" null null))
          ;;[1 1 1] AreaCollisionを配置
          (for _array_element_8 (`SceneComponent.GetChildrenComponents` (`self.AreaCollisions`) false)
            (`|SpawnActorFromClass` "/Game/MyGame/BluePrints/AI/BP_AreaCollision.BP_AreaCollision_C" (`SceneComponent.K2_GetComponentToWorld` _array_element_8) "AlwaysSpawn" "OverrideRootScale" null null))
          ;;[1 1 1] WalkerNorCrowdを配置
          (for _array_element_9 (`SceneComponent.GetChildrenComponents` (`self.Walkers`) false)
            (`|SpawnActorFromClass` "/Game/MyGame/BluePrints/AI/BP_WalkerNotCrowd.BP_WalkerNotCrowd_C" (`SceneComponent.K2_GetComponentToWorld` _array_element_9) "AlwaysSpawn" "OverrideRootScale" null null))
          (for _array_element_10 (`SceneComponent.GetChildrenComponents` (`self.Signals`) false)
            (bind _returnvalue (`SceneComponent.K2_GetComponentToWorld` _array_element_10))
            (`|SpawnActorFromClass` "/Game/MyGame/BluePrints/Car/BP_InterSection.BP_InterSection_C" (`KismetMathLibrary.MakeTransform` (`KismetMathLibrary.MakeVector` (.x (.location _returnvalue)) (.y (.location _returnvalue)) 100.0) (.rotation _returnvalue) (0.75 0.75 0.75)) "AlwaysSpawn" "OverrideRootScale" null null))
          (for _array_element_11 (`SceneComponent.GetChildrenComponents` (`self.Cars`) false)
            (`|SpawnActorFromClass` "/Game/MyGame/BluePrints/Car/BP_CarSpline.BP_CarSpline_C" (`SceneComponent.K2_GetComponentToWorld` _array_element_11) "AlwaysSpawn" "OverrideRootScale" null null))
          (for _array_element_12 (`SceneComponent.GetChildrenComponents` (`self.UpdateCarCollisions`) false)
            (`|SpawnActorFromClass` "/Game/MyGame/BluePrints/Car/BP_UpdateCarArea.BP_UpdateCarArea_C" (`SceneComponent.K2_GetComponentToWorld` _array_element_12) "AlwaysSpawn" "OverrideRootScale" null null))))
      ;[1 1 1] 親子付けを解除
      (`SceneComponent.K2_DetachFromComponent` (`self.AreaCollisions`) "KeepWorld" "KeepWorld" "KeepWorld" true)
      (`SceneComponent.K2_DetachFromComponent` (`self.WayPoints`) "KeepWorld" "KeepWorld" "KeepWorld" true)
      (`SceneComponent.K2_DetachFromComponent` (`self.Walkers`) "KeepWorld" "KeepWorld" "KeepWorld" true)
      (`SceneComponent.K2_DetachFromComponent` (`self.Signals`) "KeepWorld" "KeepWorld" "KeepWorld" true)
      (`SceneComponent.K2_DetachFromComponent` (`self.Cars`) "KeepWorld" "KeepWorld" "KeepWorld" true)
      (`SceneComponent.K2_DetachFromComponent` (`self.UpdateCarCollisions`) "KeepWorld" "KeepWorld" "KeepWorld" true))))

(fn `UserConstructionScript`)