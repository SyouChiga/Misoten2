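; BP_WalkerCrowd is a pedestrian that walks at a randomized speed and obeys walker traffic signals.
; Tick checks capsule overlaps for an opposite-facing BP_WalkerSignal, walking on blue when crossing is allowed and otherwise stopping.
; It also compares squared distance to the cached BP_Player, replacing itself with a BP_WalkerNotCrowd beyond CrowdChangeLength, a distance-based swap between walker variants.
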(event `self.ReceiveBeginPlay`
  (`parent.ReceiveBeginPlay`)
  ;[1 1 1] 歩行者のSpeedランダムに変更
  (set `CharacterMovementComponent.MaxWalkSpeed` (`KismetMathLibrary.RandomFloatInRange` 120.0 170.0) (`self.CharacterMovement`)))

(event `self.ReceiveTick`
  (params (DeltaSeconds :type "Float (single-precision)"))
  (bind _charactermovement (`self.CharacterMovement`))
  (bind _overlappingactors (`PrimitiveComponent.GetOverlappingActors` (`self.Capsule`) "/Game/MyGame/BluePrints/Car/WalkerSignals/BP_WalkerSignal.BP_WalkerSignal_C"))
  (bind _returnvalue (`SceneComponent.K2_GetComponentToWorld` (`self.Mesh`)))
  (`parent.ReceiveTick` DeltaSeconds)
  (`|ExecutionSequence`
    (:`then_0`
      (`/Engine/EditorBlueprintResources/StandardMacros.DoOnce` false
        (:`Completed`
          ;[1 1 1] Player取得
          (bind _outactors (`GameplayStatics.GetAllActorsOfClass` "/Game/MyGame/BluePrints/Player/BP_Player.BP_Player_C"))
          (set `self.Player` (`|GetArrayItem` _outactors)))))
    (:`then_1`
      (if (> (`KismetArrayLibrary.Array_Length` _overlappingactors) 0)
        (bind _asbp_walker_signal (cast `/Game/MyGame/BluePrints/Car/WalkerSignals/BP_WalkerSignal` (`|GetArrayItem` _overlappingactors)))
        (set `self.SignalWalker` _asbp_walker_signal)
        (if (< (`KismetMathLibrary.Dot_VectorVector` (`SceneComponent.GetForwardVector` (`self.Forward`)) (`SceneComponent.GetForwardVector` (`/Game/MyGame/BluePrints/Car/WalkerSignals/BP_WalkerSignal.Arrow` (`self.SignalWalker`)))) 0.0)
          (if (`/Game/MyGame/BluePrints/Car/WalkerSignals/BP_WalkerSignal.CanCross` (`self.SignalWalker`))
            (switch `/Game/MyGame/BluePrints/Car/ENUM_SignalColor` (`/Game/MyGame/BluePrints/Car/WalkerSignals/BP_WalkerSignal.SignalColor` (`self.SignalWalker`))
              (:`NewEnumerator0`
                (set `CharacterMovementComponent.MaxWalkSpeed` 150.0 _charactermovement))
              (:`NewEnumerator1`
                (set `CharacterMovementComponent.MaxWalkSpeed` 0.0 _charactermovement :!label _label))
              (:`NewEnumerator2`
                (goto _label)))
            (else
              (goto _label))))))
    (:`then_2`
      ;[1 1 1] Playerとの距離を見て一定以上だった場合、NotCrowdをスポーンし、自分を破棄
      (if (> (`KismetMathLibrary.VSizeSquared` (- (`self.K2_GetActorLocation` (`self.Player`)) (`self.K2_GetActorLocation`))) (`KismetMathLibrary.Square` (`self.CrowdChangeLength`)))
        (`|SpawnActorFromClass` "/Game/MyGame/BluePrints/AI/BP_WalkerNotCrowd.BP_WalkerNotCrowd_C" (`KismetMathLibrary.MakeTransform` (`KismetMathLibrary.MakeVector` (.x (.location _returnvalue)) (.y (.location _returnvalue)) 160.0) (.rotation _returnvalue) (.scale _returnvalue)) "Undefined" "OverrideRootScale" null null)
        (`self.K2_DestroyActor`)))))

(fn `UserConstructionScript`
  (`parent.UserConstructionScript`))