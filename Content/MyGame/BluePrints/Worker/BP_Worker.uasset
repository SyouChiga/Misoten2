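; BP_Worker is a worker dispatched to an Accident to resolve it, driven by a State switch on Tick.
; It spawns with a random XY offset, steers toward the Accident, and sidesteps other workers by turning on a forward line-trace hit.
; Tagged-collision overlap, or prolonged blocking within range, sets IsAproach, which stops movement.
; Working feeds WorkSpeed into the Accident; a missing Accident leads to Station destroying the worker.
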(event `self.ReceiveBeginPlay`
  (bind (_returnvalue_x _returnvalue_y _returnvalue_z) (`KismetMathLibrary.BreakVector` (`self.K2_GetActorLocation`)))
  ;[1 1 1] Spawn時に座標を変更
  (`self.K2_SetActorLocation` (`KismetMathLibrary.MakeVector` (+ _returnvalue_x (`KismetMathLibrary.RandomFloatInRange` -500.0 500.0)) (+ _returnvalue_y (`KismetMathLibrary.RandomFloatInRange` -500.0 500.0)) _returnvalue_z) true))

(event `self.ReceiveTick`
  (params (DeltaSeconds :type "Float (single-precision)"))
  (bind _returnvalue (`self.K2_GetActorLocation`))
  (bind (_returnvalue_roll _returnvalue_pitch _returnvalue_yaw) (`KismetMathLibrary.BreakRotator` (`self.K2_GetActorRotation`)))
  (bind (_returnvalue_roll_2 _returnvalue_pitch_2 _returnvalue_yaw_2) (`KismetMathLibrary.BreakRotator` (`KismetMathLibrary.RInterpTo` (`self.K2_GetActorRotation`) (`KismetMathLibrary.FindLookAtRotation` (`self.K2_GetActorLocation`) (`self.K2_GetActorLocation` (`self.Accident`))) (`GameplayStatics.GetWorldDeltaSeconds`) 25.0)))
  (bind (_returnvalue_roll_3 _returnvalue_pitch_3 _returnvalue_yaw_3) (`KismetMathLibrary.BreakRotator` (`KismetMathLibrary.RInterpTo` (`self.K2_GetActorRotation`) (`KismetMathLibrary.FindLookAtRotation` (`self.K2_GetActorLocation`) (`self.K2_GetActorLocation` (`self.Accident`))) (`GameplayStatics.GetWorldDeltaSeconds`) 25.0)))
  (switch `/Game/MyGame/BluePrints/Worker/ENUM_WorkerState` (`self.State`)
    (:`NewEnumerator0`
      (if (not (`self.IsAproach`))
        (`|ExecutionSequence`
          (:`then_0`
            ;[1 1 1] 出動先アクシデントの存在チェック
            (`/Engine/EditorBlueprintResources/StandardMacros.IsValid` (`self.Accident`)
              (:`Is Valid`
                ;[1 1 1] 自身からRayを飛ばしてWorkerに当たった場合回避するようにする
                (bind _outhit (`KismetSystemLibrary.LineTraceSingle` _returnvalue (+ _returnvalue (* (`self.GetActorForwardVector`) 200.0)) "TraceTypeQuery1"))
                (cast `/Game/MyGame/BluePrints/Worker/BP_Worker` (`.HitActor` (`GameplayStatics.BreakHitResult` _outhit))
                  (:`then`
                    (`|ExecutionSequence`
                      (:`then_0`
                        ;;[1 1 1] 最初の1フレーム目で左に曲がるか右に曲がるかランダムに決める
                        (`/Engine/EditorBlueprintResources/StandardMacros.DoOnce` false
                          (:`Completed`
                            (if (`KismetMathLibrary.RandomBool`)
                              (set `self.HittingRotate` -1.0)
                              (else
                                (set `self.HittingRotate` 1.0))))))
                      (:`then_1`
                        ;;[1 1 1] ヒットし続けている場合、体を回転し続ける
                        (`self.K2_SetActorRotation` (`KismetMathLibrary.MakeRotator` _returnvalue_roll _returnvalue_pitch (+ _returnvalue_yaw (`self.HittingRotate`))))
                        ;[1 1 1] Workerが60フレームつっかかってて、WorkingRange内に入っている場合、WorkingにStateを変化する
                        (bind _result (`/Engine/EditorBlueprintResources/StandardMacros.IncrementInt` (`self.HittingCount`))
                          (:`  `
                            (if (> _result 60)
                              (if (< (`KismetMathLibrary.VSizeSquared` (- (`self.K2_GetActorLocation` (`self.Accident`)) (`self.K2_GetActorLocation`))) (`KismetMathLibrary.Square` (`self.WorkingRange`)))
                                (set `self.IsAproach` true))))))))
                  (:`CastFailed`
                    ;[1 1 1] 前進
                    (`self.AddMovementInput` (`self.GetActorForwardVector`))
                    ;[1 1 1] Accidentを向く
                    (`self.K2_SetActorRotation` (`KismetMathLibrary.MakeRotator` 0.0 0.0 _returnvalue_yaw_2)))))
              (:`Is Not Valid`
                (set `self.State` "NewEnumerator2")))))
        (else
          ;[1 1 1] Accidentを向く
          (`self.K2_SetActorRotation` (`KismetMathLibrary.MakeRotator` 0.0 0.0 _returnvalue_yaw_3)))))
    (:`NewEnumerator1`
      ;[1 1 1] 出動先アクシデントの存在チェック
      (`/Engine/EditorBlueprintResources/StandardMacros.IsValid` (`self.Accident`)
        (:`Is Valid`
          (`/Game/MyGame/BluePrints/Accident/BP_Accident.Resolving` (`self.Accident`) (`self.WorkSpeed`)))
        (:`Is Not Valid`
          (set `self.State` "NewEnumerator2"))))
    (:`NewEnumerator2`
      (`/Game/MyGame/BluePrints/Station/BP_Station.DestroyWorker` (`self.Station`) self))))

(event `self.CapsuleComponent.OnComponentBeginOverlap`
  (params (OverlappedComponent :type "PrimitiveComponent Object Reference") (OtherActor :type "Actor Object Reference") (OtherComp :type "PrimitiveComponent Object Reference") (OtherBodyIndex :type Integer) (bFromSweep :type Boolean) (SweepResult :type "HitResult Structure (by ref)"))
  (bind (_returnvalue_roll _returnvalue_pitch _returnvalue_yaw) (`KismetMathLibrary.BreakRotator` (`KismetMathLibrary.FindLookAtRotation` (`self.K2_GetActorLocation`) (`self.K2_GetActorLocation` OtherActor))))
  (switch `/Game/MyGame/BluePrints/Worker/ENUM_WorkerState` (`self.State`)
    (:`NewEnumerator0`
      ;[1 1 1] Accident到達
      (if (== (`self.Accident`) OtherActor)
        (if (`ActorComponent.ComponentHasTag` OtherComp "WorkerCollision")
          (`self.K2_SetActorRotation` (`KismetMathLibrary.MakeRotator` 0.0 0.0 _returnvalue_yaw))
          (set `self.IsAproach` true))))))

(fn `GetState`
  (returns (State :type "/Game/MyGame/BluePrints/Worker/ENUM_WorkerState Enum"))
  (return (`self.State`)))

(fn `RandomWalk`
  (set `self.RandomWalkDelay` (+ (`self.RandomWalkDelay`) (`GameplayStatics.GetWorldDeltaSeconds`)))
  (`self.K2_AddActorLocalRotation` (`KismetMathLibrary.MakeRotator` 0.0 0.0 (`self.RandomWalkDegree`)))
  (if (>= (`self.RandomWalkDelay`) (`self.RandomWalkDelayValue`))
    (set `self.RandomWalkDelay` 0.0)
    (set `self.RandomWalkDelayValue` (`KismetMathLibrary.RandomFloatInRange` (`self.RandomWalkTimeMin`) (`self.RandomWalkTimeMax`)))
    (set `self.RandomWalkDegree` (`KismetMathLibrary.RandomFloatInRange` -20.0 20.0))))

(fn `UserConstructionScript`)