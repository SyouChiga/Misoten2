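; Accident generator that periodically spawns fire accidents at random spots on a square field centred on the world origin.
; Tick accumulates time and, at each interval, rolls one of two probabilities depending on whether any accidents are active.
; Placement retries random points to avoid the central radius, but the spawn re-rolls its location, so that check is not applied.
; Spawned accidents receive a generator reference and are tracked in an array until DestroyAccident removes them.
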(event `self.ReceiveTick`
  (params (DeltaSeconds :type "Float (single-precision)"))
  (set `self.Delay` (+ DeltaSeconds (`self.Delay`)))
  (if (< (`self.DelayValue`) (`self.Delay`))
    (set `self.Delay` 0.0)
    (if (== (`KismetArrayLibrary.Array_Length` (`self.Accidents`)) 0)
      (if (< (`KismetMathLibrary.RandomFloatInRange` 0.0 100.0) (`self.NoAccidentProbability`))
        (`self.SpawnAccidentRandom` "/Game/MyGame/BluePrints/BP_FireAccident.BP_FireAccident_C" :!label _label))
      (elif (< (`KismetMathLibrary.RandomFloatInRange` 0.0 100.0) (`self.OneAccidentProbability`))
        (goto _label)))))

(fn `DestroyAccident`
  (params (Accident :type "/Game/MyGame/BluePrints/BP_Accident Object Reference (by ref)"))
  (`KismetArrayLibrary.Array_RemoveItem` (`self.Accidents`) Accident)
  (`self.K2_DestroyActor` Accident))

(fn `SpawnAccident`
  (params (AccidentClass :type "/Game/MyGame/BluePrints/BP_Accident Class Reference") (Location :type "Vector Structure"))
  (bind _returnvalue (`|SpawnActorFromClass` AccidentClass (`KismetMathLibrary.MakeTransform` Location) "AlwaysSpawn" "OverrideRootScale" null self null))
  (`KismetArrayLibrary.Array_Add` (`self.Accidents`) _returnvalue))

(fn `SpawnAccidentRandom`
  (params (AccidentClass :type "/Game/MyGame/BluePrints/BP_Accident Class Reference"))
  (bind _returnvalue (/ (`self.FieldWidthDepth`) 2.0))
  (bind _returnvalue_2 (* _returnvalue -1.0))
  (bind _returnvalue_3 (`KismetMathLibrary.RandomFloatInRange` _returnvalue_2 _returnvalue))
  (bind _returnvalue_4 (`KismetMathLibrary.RandomFloatInRange` _returnvalue_2 _returnvalue))
  (for _ (range 11)
    (if (>= (`KismetMathLibrary.VSize` (`KismetMathLibrary.MakeVector` _returnvalue_4 _returnvalue_3 10.0)) 350.0)
      (break)))
  (`self.SpawnAccident` AccidentClass (`KismetMathLibrary.MakeVector` _returnvalue_4 _returnvalue_3 10.0)))

(fn `UserConstructionScript`)