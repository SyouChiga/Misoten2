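; Camera spline actor that builds a curved path between two audience actors, presumably for camera moves from one to the other.
; On BeginPlay it sets a two-point world-space spline from the start audience's CameraPoint to the end audience's SplinePoint.
; Each endpoint tangent follows that audience's forward vector, scaled by half the distance between the two CameraPoints, so the curve adapts to their spacing.
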(event `self.ReceiveBeginPlay`
  (bind _endaudience (`self.EndAudience`))
  (bind _returnvalue (`SceneComponent.K2_GetComponentLocation` (`/Game/MyGame/BluePrints/Audience/BP_Audience.CameraPoint` (`self.StartAudience`))))
  (bind _returnvalue_2 (* (`KismetMathLibrary.VSize` (- _returnvalue (`SceneComponent.K2_GetComponentLocation` (`/Game/MyGame/BluePrints/Audience/BP_Audience.CameraPoint` _endaudience)))) 0.5))
  ;[1 1 1] Spline始点終点と接線設定
  (`SplineComponent.SetSplinePoints` (`self.Spline`) (`|MakeArray` _returnvalue (`SceneComponent.K2_GetComponentLocation` (`/Game/MyGame/BluePrints/Audience/BP_Audience.SplinePoint` _endaudience))) "World" true)
  (`|ExecutionSequence`
    (:`then_0`
      (`SplineComponent.SetTangentAtSplinePoint` (`self.Spline`) 0 (* (`self.GetActorForwardVector` (`self.StartAudience`)) _returnvalue_2) "World" true))
    (:`then_1`
      (`SplineComponent.SetTangentAtSplinePoint` (`self.Spline`) 1 (* (`self.GetActorForwardVector` (`self.EndAudience`)) _returnvalue_2) "World" true))))

(fn `UserConstructionScript`)