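; BP_CameraSpline is an audience-related spline actor that spans from the base's camera point to an audience location.
; Its construction script pins the first spline point to the CameraPoint of the first BP_Base found and the last point to the AudienceLocation actor, in world space.
; The endpoints update only when AudienceLocation is valid, with no check that a BP_Base exists.
; The event graph holds no active logic.
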(fn `UserConstructionScript`
  (bind _outactors (`GameplayStatics.GetAllActorsOfClass` "/Game/MyGame/BluePrints/BP_Base.BP_Base_C"))
  (`/Engine/EditorBlueprintResources/StandardMacros.IsValid` (`self.AudienceLocation`)
    (:`Is Valid`
      ;[1 1 1] Spline始点設定
      (`SplineComponent.SetLocationAtSplinePoint` (`self.Spline`) 0 (`SceneComponent.K2_GetComponentLocation` (`/Game/MyGame/BluePrints/BP_Base.CameraPoint` (`|GetArrayItem` _outactors))) "World" true)
      ;[1 1 1] Spline終点設定
      (`SplineComponent.SetLocationAtSplinePoint` (`self.Spline`) (- (`SplineComponent.GetNumberOfSplinePoints` (`self.Spline`)) 1) (`self.K2_GetActorLocation` (`self.AudienceLocation`)) "World" true))))