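; BP_Walker is an AI-driven walker that can stop to look at accidents and display a first-discoverer sign.
; On BeginPlay it gathers all BP_WayPoint actors and runs its BehaviorTree.
; LookAccident stores the accident and state, calling the player's VisibleDispatch if this walker is the player's Parent.
; Tick returns it to Walking once the accident becomes invalid, hiding the sign and calling HiddenDispatch without that Parent check.
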(event `self.ReceiveBeginPlay`
  ;[1 1 1] ワールドに配置したWayPointを配列にセット
  (bind _outactors (`GameplayStatics.GetAllActorsOfClass` "/Game/MyGame/BluePrints/AI/BP_WayPoint.BP_WayPoint_C"))
  (set `self.WayPoints` _outactors)
  ;[1 1 1] BehaviorTree登録
  (`AIController.RunBehaviorTree` (`AIBlueprintHelperLibrary.GetAIController` self) (`self.BehaviorTree`)))

(event `self.ReceiveTick`
  (params (DeltaSeconds :type "Float (single-precision)"))
  (`|ExecutionSequence`
    (:`then_0`
      (`/Engine/EditorBlueprintResources/StandardMacros.DoOnce` false
        (:`Completed`
          (bind _asbp_player (cast `/Game/MyGame/BluePrints/Player/BP_Player` (`GameplayStatics.GetPlayerPawn` 0)))
          (set `self.Player` _asbp_player))))
    (:`then_1`
      (switch `/Game/MyGame/BluePrints/Walker/ENUM_WalkerState` (`self.State`)
        (:`NewEnumerator1`
          ;[1 1 1] Accident注目中
          (`/Engine/EditorBlueprintResources/StandardMacros.IsValid` (`self.LookingAccident`)
            (:`Is Not Valid`
              (set `self.State` "NewEnumerator0")
              (`/Game/MyGame/BluePrints/Player/BP_Player.HiddenDispatch` (`self.Player`))
              (`SceneComponent.SetVisibility` (`self.FirstDiscovererSign`) false false))))))))

(fn `BecomeFirstDiscoverer`
  (`SceneComponent.SetVisibility` (`self.FirstDiscovererSign`) true false))

(fn `LookAccident`
  (params (LookingAccident :type "/Game/MyGame/BluePrints/Accident/BP_Accident Object Reference"))
  (`|ExecutionSequence`
    (:`then_0`
      (`/Engine/EditorBlueprintResources/StandardMacros.IsValid` (`self.Player`)
        (:`Is Not Valid`
          (bind _asbp_player (cast `/Game/MyGame/BluePrints/Player/BP_Player` (`GameplayStatics.GetPlayerPawn` 0)))
          (set `self.Player` _asbp_player))))
    (:`then_1`
      (set `self.LookingAccident` LookingAccident)
      (set `self.State` "NewEnumerator1")
      (bind _asbp_walker (cast `/Game/MyGame/BluePrints/Walker/BP_Walker` (`/Game/MyGame/BluePrints/Player/BP_Player.Parent` (`self.Player`))))
      (if (== _asbp_walker self)
        (`/Game/MyGame/BluePrints/Player/BP_Player.VisibleDispatch` (`self.Player`))))))

(fn `UserConstructionScript`)