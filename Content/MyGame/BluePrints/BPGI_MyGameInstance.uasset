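; Game instance Blueprint that owns a screen fade widget shared across the game.
; Init creates the BPW_NormalFade widget once and stores it for reuse.
; Helper functions add it to the viewport, fade out by playing its AlphaIncrease animation, fade in by playing that same animation in reverse, and report whether the fade is still playing.
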(event `self.ReceiveInit`
  (bind _returnvalue (`|CreateWidget` "/Game/MyGame/BluePrints/BPW_NormalFade.BPW_NormalFade_C" null self))
  (set `self.NormalFadeWidget` _returnvalue))

(fn `IsPlayingNormalFadeAnimation`
  (returns (IsPlaying :type Boolean))
  (bind _normalfadewidget (`self.NormalFadeWidget`))
  (return (`UserWidget.IsAnimationPlaying` _normalfadewidget (`/Game/MyGame/BluePrints/BPW_NormalFade.AlphaIncrease` _normalfadewidget))))

(fn `NormalFadeAddToViewport`
  (`UserWidget.AddToViewport` (`self.NormalFadeWidget`) 0))

(fn `StartNormalFadeIn`
  (bind _normalfadewidget (`self.NormalFadeWidget`))
  (`UserWidget.PlayAnimation` _normalfadewidget (`/Game/MyGame/BluePrints/BPW_NormalFade.AlphaIncrease` _normalfadewidget) 0.0 1 "Reverse" 1.0))

(fn `StartNormalFadeOut`
  (bind _normalfadewidget (`self.NormalFadeWidget`))
  (`UserWidget.PlayAnimation` _normalfadewidget (`/Game/MyGame/BluePrints/BPW_NormalFade.AlphaIncrease` _normalfadewidget) 0.0 1 "Forward" 1.0))