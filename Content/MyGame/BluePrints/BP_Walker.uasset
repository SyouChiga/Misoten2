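; BP_Walker is a wandering pedestrian character that stops to watch accidents it comes across.
; While walking, Tick moves it forward and applies a random yaw turn whenever a delay timer expires, and capsule hits turn it along the hit normal.
; Overlapping a BP_Accident component tagged WalkerCollision switches its state to looking, so it faces that accident until it becomes invalid, then resumes walking.
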(event `self.ReceiveTick`
  (params (DeltaSeconds :type "Float (single-precision)"))
  (bind (_returnvalue_roll _returnvalue_pitch _returnvalue_yaw) (`KismetMathLibrary.BreakRotator` (`KismetMathLibrary.FindLookAtRotation` (`self.K2_GetActorLocation`) (`self.K2_GetActorLocation` (`self.LookingAccident`)))))
  (switch `/Game/MyGame/BluePrints/ENUM_WalkerState` (`self.State`)
    (:`NewEnumerator0`
      ;[1 1 1] 前進
      (`self.AddMovementInput` (`self.GetActorForwardVector`))
      ;[1 1 1] ランダム方向転換
      (set `self.RandomTurnDelay` (+ (`self.RandomTurnDelay`) (`GameplayStatics.GetWorldDeltaSeconds`)))
      (if (>= (`self.RandomTurnDelay`) (`self.RandomTurnDelayThreshold`))
        (set `self.RandomTurnDelay` 0.0)
        (`self.K2_AddActorWorldRotation` (`KismetMathLibrary.MakeRotator` 0.0 0.0 (`KismetMathLibrary.RandomFloatInRange` -180.0 180.0)))))
    (:`NewEnumerator1`
      ;[1 1 1] Accident注目中
      (`/Engine/EditorBlueprintResources/StandardMacros.IsValid` (`self.LookingAccident`)
        (:`Is Valid`
          (`self.K2_SetActorRotation` (`KismetMathLibrary.MakeRotator` 0.0 0.0 _returnvalue_yaw)))
        (:`Is Not Valid`
          (set `self.State` "NewEnumerator0"))))))

(event `self.CapsuleComponent.OnComponentHit`
  (params (HitComponent :type "PrimitiveComponent Object Reference") (OtherActor :type "Actor Object Reference") (OtherComp :type "PrimitiveComponent Object Reference") (NormalImpulse :type "Vector Structure") (Hit :type "HitResult Structure (by ref)"))
  (bind (_returnvalue_roll _returnvalue_pitch _returnvalue_yaw) (`KismetMathLibrary.BreakRotator` (`KismetMathLibrary.FindLookAtRotation` Hit_Location (+ Hit_Location Hit_Normal))))
  ;[1 1 1] 何かとぶつかった時反転
  (`self.K2_SetActorRotation` (`KismetMathLibrary.MakeRotator` 0.0 0.0 _returnvalue_yaw)))

(event `self.CapsuleComponent.OnComponentBeginOverlap`
  (params (OverlappedComponent :type "PrimitiveComponent Object Reference") (OtherActor :type "Actor Object Reference") (OtherComp :type "PrimitiveComponent Object Reference") (OtherBodyIndex :type Integer) (bFromSweep :type Boolean) (SweepResult :type "HitResult Structure (by ref)"))
  ;[1 1 1] Accident発見
  (bind _asbp_accident (cast `/Game/MyGame/BluePrints/BP_Accident` OtherActor))
  (if (`ActorComponent.ComponentHasTag` OtherComp "WalkerCollision")
    (set `self.LookingAccident` _asbp_accident)
    (set `self.State` "NewEnumerator1")))

(fn `UserConstructionScript`)