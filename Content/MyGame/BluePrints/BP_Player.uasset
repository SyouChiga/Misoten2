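; BP_Player is a first-person camera that jumps between mobs and bases the player looks at.
; ChangeCamera line-traces from screen center, ignoring the current host, then attaches the player to the hit BP_Mob or BP_Base's CameraPoint and sets CameraState.
; Look input rotates the camera with limited pitch, and limits yaw only in Mob state.
; Horizontal look also resets roll to zero after each rotation.
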(event `InputAxis|LookRight`
  (params (AxisValue :type "Float (single-precision)"))
  (bind _camera (`self.Camera`))
  (bind _moblookrightlimit (`self.MobLookRightLimit`))
  (bind _returnvalue (`SceneComponent.GetRelativeTransform` _camera))
  (bind _returnvalue_2 (`SceneComponent.GetRelativeTransform` (`self.Camera`)))
  ;[1 1 1] 主観視点カメラ
  (switch `/Game/MyGame/BluePrints/ENUM_PlayerCameraState` (`self.CameraState`)
    (:`NewEnumerator0`
      ;;[1 1 1] ベース時制限無し
      (`SceneComponent.K2_AddLocalRotation` (`self.Camera`) (`KismetMathLibrary.MakeRotator` 0.0 0.0 AxisValue) false false)
      ;;[1 1 1] Roll対策
      (`SceneComponent.K2_SetRelativeRotation` _camera (`KismetMathLibrary.MakeRotator` 0.0 (.pitch (.rotation _returnvalue)) (.yaw (.rotation _returnvalue))) false false :!label _label))
    (:`NewEnumerator1`
      ;;[1 1 1] Mob時左右角度制限
      (if (>= AxisValue 0.0)
        (if (<= (.yaw (.rotation _returnvalue_2)) _moblookrightlimit)
          (`SceneComponent.K2_AddLocalRotation` (`self.Camera`) (`KismetMathLibrary.MakeRotator` 0.0 0.0 AxisValue) false false :!label _label_2)
          (goto _label))
        (elif (>= (.yaw (.rotation _returnvalue_2)) (* _moblookrightlimit -1.0))
          (goto _label_2))))))

(event `InputAxis|LookUp`
  (params (AxisValue :type "Float (single-precision)"))
  (bind _lookuplimit (`self.LookUpLimit`))
  (bind _returnvalue (`SceneComponent.GetRelativeTransform` (`self.Camera`)))
  ;[1 1 1] 主観視点カメラ
  ;;[1 1 1] 上下角度制限
  (if (>= AxisValue 0.0)
    (if (<= (.pitch (.rotation _returnvalue)) _lookuplimit)
      (`SceneComponent.K2_AddLocalRotation` (`self.Camera`) (`KismetMathLibrary.MakeRotator` 0.0 AxisValue) false false :!label _label_3))
    (elif (>= (.pitch (.rotation _returnvalue)) (* _lookuplimit -1.0))
      (goto _label_3))))

(event `InputAction|ChangeCamera`
  (params (Key :type "Key Structure"))
  (bind _camera (`self.Camera`))
  (bind _returnvalue (`SceneComponent.K2_GetComponentLocation` _camera))
  ;[1 1 1] 画面中心に捉えたモブまたはベースに乗り移る
  (:`Pressed`
    (bind _outhit (`KismetSystemLibrary.LineTraceSingle` _returnvalue (+ _returnvalue (* (`SceneComponent.GetForwardVector` _camera) (`self.LineTraceLength`))) "TraceTypeQuery1" false (`|MakeArray` (`self.Parent`))))
    (`|ExecutionSequence`
      (:`then_0`
        ;;[1 1 1] モブに乗り移り
        (bind _asbp_mob (cast `/Game/MyGame/BluePrints/BP_Mob` (`.HitActor` (`GameplayStatics.BreakHitResult` _outhit))))
        (set `self.Parent` (`.HitActor` (`GameplayStatics.BreakHitResult` _outhit)))
        (`self.K2_AttachToComponent` (`/Game/MyGame/BluePrints/BP_Mob.CameraPoint` _asbp_mob) "None" "KeepRelative" "KeepRelative" "KeepRelative")
        (`self.K2_SetActorRelativeLocation` (0.0 0.0 0.0))
        (`SceneComponent.K2_SetRelativeRotation` :`self` (`self.Camera`))
        (set `self.CameraState` "NewEnumerator1"))
      (:`then_1`
        ;;[1 1 1] ベースに乗り移り
        (bind _asbp_base (cast `/Game/MyGame/BluePrints/BP_Base` (`.HitActor` (`GameplayStatics.BreakHitResult` _outhit))))
        (set `self.Parent` (`.HitActor` (`GameplayStatics.BreakHitResult` _outhit)))
        (`self.K2_AttachToComponent` (`/Game/MyGame/BluePrints/BP_Base.CameraPoint` _asbp_base) "None" "KeepRelative" "KeepRelative" "KeepRelative")
        (`self.K2_SetActorRelativeLocation` (0.0 0.0 0.0))
        (`SceneComponent.K2_SetRelativeRotation` :`self` (`self.Camera`))
        (set `self.CameraState` "NewEnumerator0")))))

(fn `UserConstructionScript`)