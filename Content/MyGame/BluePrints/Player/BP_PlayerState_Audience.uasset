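; Player state for viewing through a BP_Audience's camera, where the player hops to other audiences or dispatches workers to that audience's accident.
; BeginPlay snaps to its CameraPoint and toggles dispatch UI.
; Tick rebuilds selectable audiences from collision overlaps, screen checks and line traces, auto-updating selection, or returns to base if the parent is invalid.
; Input events cycle selection, transition states, or spawn fire or police workers by UI choice.
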(event `self.ReceiveTick`
  (params (DeltaSeconds :type "Float (single-precision)"))
  (bind _player (`self.Player`))
  (bind _selectingaudience_audience (break `/Game/MyGame/BluePrints/Player/STRUCT_SelectableAudience` (`/Game/MyGame/BluePrints/Player/BP_Player.SelectingAudience` (`self.Player`))))
  (`/Engine/EditorBlueprintResources/StandardMacros.IsValid` (`/Game/MyGame/BluePrints/Player/BP_Player.Parent` (`self.Player`))
    (:`Is Valid`
      (`|ExecutionSequence`
        (:`then_0`
          ;[1 1 1] 選択可能な画面内Walkerの検出
          (`/Game/MyGame/BluePrints/Player/BP_Player.ClearSelectableAudiences` (`self.Player`))
          (for _array_element (`PrimitiveComponent.GetOverlappingActors` (`/Game/MyGame/BluePrints/Player/BP_Player.ChangeCameraCollision` (`self.Player`)) "/Game/MyGame/BluePrints/Audience/BP_Audience.BP_Audience_C")
            ;;[1 1 1] 画面内判定
            (bind _returnvalue (`/Game/MyGame/BluePrints/Player/BP_Player.JudgeIsOnScreen` (`self.Player`) _array_element))
            (if _returnvalue
              ;;[1 1 1] LineTraceでSelfと目的のActorとの遮蔽を判定
              (bind _returnvalue_2 (`/Game/MyGame/BluePrints/Player/BP_Player.JudgeIsMatchActorLineTrace` (`self.Player`) _array_element))
              (if _returnvalue_2
                (bind _asbp_audience (cast `/Game/MyGame/BluePrints/Audience/BP_Audience` _array_element))
                (`/Game/MyGame/BluePrints/Player/BP_Player.AddSelectableAudience` (`self.Player`) _asbp_audience)))))
        (:`then_1`
          ;[1 1 1] 選択しているWalkerの自動切換え
          ;;[1 1 1] 選択中のWalkerの有無
          (`/Engine/EditorBlueprintResources/StandardMacros.IsValid` _selectingaudience_audience
            (:`Is Valid`
              ;;[1 1 1] 選択中のWalkerが画面内に残っているか判定
              (bind _isexist (`/Game/MyGame/BluePrints/Player/BP_Player.IsExistSelectingAudienceInSelectableAudiences` (`self.Player`)))
              (if (not _isexist)
                ;;[1 1 1] 画面内に他のWalkerが存在する場合、画面上で最も近いWalkerを選択
                (if (> (`KismetArrayLibrary.Array_Length` (`/Game/MyGame/BluePrints/Player/BP_Player.SelectableAudiences` (`self.Player`))) 0)
                  (`/Game/MyGame/BluePrints/Player/BP_Player.SelectNearAudienceOnScreen` (`self.Player`))
                  (else
                    (`/Game/MyGame/BluePrints/Player/BP_Player.SetSelectingAudience` :`self` (`self.Player`))))))
            (:`Is Not Valid`
              ;;[1 1 1] 選択可能なWalkerがいる場合選択する
              (if (> (`KismetArrayLibrary.Array_Length` (`/Game/MyGame/BluePrints/Player/BP_Player.SelectableAudiences` (`self.Player`))) 0)
                (`/Game/MyGame/BluePrints/Player/BP_Player.SetSelectingAudience` (`self.Player`) (`|GetArrayItem` (`/Game/MyGame/BluePrints/Player/BP_Player.SelectableAudiences` (`self.Player`))))))))))
    (:`Is Not Valid`
      (`/Game/MyGame/BluePrints/Player/BP_Player.ChangeState` _player "/Game/MyGame/BluePrints/Player/BP_PlayerState_AudienceToBase.BP_PlayerState_AudienceToBase_C" (`/Game/MyGame/BluePrints/Player/BP_Player.State` _player)))))

(event `self.ReceiveBeginPlay`
  (bind _player (`self.Player`))
  (`/Game/MyGame/BluePrints/Player/BP_Player.SwitchToAudienceCamera` (`self.Player`))
  (bind _asbp_audience (cast `/Game/MyGame/BluePrints/Audience/BP_Audience` (`/Game/MyGame/BluePrints/Player/BP_Player.Parent` (`self.Player`))))
  (`|ExecutionSequence`
    (:`then_0`
      (bind (_returnvalue_location _returnvalue_rotation) (`KismetMathLibrary.BreakTransform` (`SceneComponent.K2_GetComponentToWorld` (`/Game/MyGame/BluePrints/Audience/BP_Audience.CameraPoint` _asbp_audience))))
      (`self.K2_SetActorTransform` (`self.Player`) (`KismetMathLibrary.MakeTransform` _returnvalue_location _returnvalue_rotation) false false))
    (:`then_1`
      (if (`/Game/MyGame/BluePrints/Audience/BP_Audience.IsCanDispatch` _asbp_audience)
        ;[1 1 1] 出動UI表示・非表示切り替え
        (`/Game/MyGame/BluePrints/Player/BP_Player.VisibleDispatch` _player)
        (else
          (`/Game/MyGame/BluePrints/Player/BP_Player.HiddenDispatch` _player))))
    (:`then_2`
      (`/Game/MyGame/BluePrints/Player/BP_Player.SetSelectingAudience` :`self` (`self.Player`)))))

(event `self.ReturnTobase`
  (bind _player (`self.Player`))
  (`/Game/MyGame/BluePrints/Player/BP_Player.ChangeState` _player "/Game/MyGame/BluePrints/Player/BP_PlayerState_AudienceToBase.BP_PlayerState_AudienceToBase_C" (`/Game/MyGame/BluePrints/Player/BP_Player.State` _player)))

(event `self.ChangeCamera`
  (bind _selectingaudience_audience (break `/Game/MyGame/BluePrints/Player/STRUCT_SelectableAudience` (`/Game/MyGame/BluePrints/Player/BP_Player.SelectingAudience` (`self.Player`))))
  (switch `/Game/MyGame/BluePrints/Stage01/Widgets/ENUM_SelectImage` (`/Game/MyGame/BluePrints/Stage01/Widgets/BPW_SelectWorker.GetSelectImg` (`/Game/MyGame/BluePrints/Player/BP_Player.SelectingWorkerUI` (`self.Player`)))
    (:`NewEnumerator3`
      (`/Engine/EditorBlueprintResources/StandardMacros.IsValid` _selectingaudience_audience
        (:`Is Valid`
          (`/Game/MyGame/BluePrints/Player/BP_Player.ChangeState` (`self.Player`) "/Game/MyGame/BluePrints/Player/BP_PlayerState_AudienceToAudience.BP_PlayerState_AudienceToAudience_C" self))))))

(event `self.Dispatch`
  (bind _asbp_audience (cast `/Game/MyGame/BluePrints/Audience/BP_Audience` (`/Game/MyGame/BluePrints/Player/BP_Player.Parent` (`self.Player`))))
  (if (`/Game/MyGame/BluePrints/Audience/BP_Audience.IsCanDispatch` _asbp_audience)
    (switch `/Game/MyGame/BluePrints/Stage01/Widgets/ENUM_SelectImage` (`/Game/MyGame/BluePrints/Stage01/Widgets/BPW_SelectWorker.GetSelectImg` (`/Game/MyGame/BluePrints/Player/BP_Player.SelectingWorkerUI` (`self.Player`)))
      (:`NewEnumerator0`
        (bind _accident (`/Game/MyGame/BluePrints/Audience/BP_Audience.Accident` _asbp_audience))
        (bind _returnvalue (`self.K2_GetActorLocation` (`/Game/MyGame/BluePrints/Accident/BP_Accident.WorkerSpawnPoint` (`/Game/MyGame/BluePrints/Audience/BP_Audience.Accident` _asbp_audience))))
        (`/Game/MyGame/BluePrints/Station/BP_Station.SpawnWorker` (`/Game/MyGame/BluePrints/Player/BP_Player.FireStation` (`self.Player`)) _accident _returnvalue))
      (:`NewEnumerator1`
        (`/Game/MyGame/BluePrints/Station/BP_Station.SpawnWorker` (`/Game/MyGame/BluePrints/Player/BP_Player.PoliceStation` (`self.Player`)) _accident _returnvalue)))))

(event `self.SelectRight`
  (if (> (`KismetArrayLibrary.Array_Length` (`/Game/MyGame/BluePrints/Player/BP_Player.SelectableAudiences` (`self.Player`))) 1)
    (`/Game/MyGame/BluePrints/Player/BP_Player.SelectRightAudience` (`self.Player`))))

(event `self.SelectLeft`
  (if (> (`KismetArrayLibrary.Array_Length` (`/Game/MyGame/BluePrints/Player/BP_Player.SelectableAudiences` (`self.Player`))) 1)
    (`/Game/MyGame/BluePrints/Player/BP_Player.SelectLeftAudience` (`self.Player`))))

(fn `UserConstructionScript`
  (`parent.UserConstructionScript`))