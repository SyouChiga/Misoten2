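; Player state that flies the camera from the base view to the selected first discoverer's Audience, then hands over to the Audience state.
; Each tick, MoveCamera advances the player along the Accident's camera spline, aiming slightly ahead and widening the FOV mid-path before easing back.
; At the spline's end it sets the player's Parent to that Audience.
; If the Audience becomes invalid, it switches to the AudienceToBase state instead.
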(event `self.ReceiveBeginPlay`
  (bind _player (`self.Player`))
  (`parent.ReceiveBeginPlay`)
  (`/Game/MyGame/BluePrints/Player/BP_Player.SwitchToMovingCamera` _player)
  (`/Game/MyGame/BluePrints/Player/BP_Player.StartMoveCamera` _player))

(event `self.ReceiveTick`
  (params (DeltaSeconds :type "Float (single-precision)"))
  (bind _player (`self.Player`))
  (bind _player_2 (`self.Player`))
  (bind _selectingfirstdiscoverer_audience (break `/Game/MyGame/BluePrints/Player/STRUCT_SelectableFirstDiscoverer` (`/Game/MyGame/BluePrints/Player/BP_Player.SelectingFirstDiscoverer` (`self.Player`))))
  (bind _selectingfirstdiscoverer_audience_2 (break `/Game/MyGame/BluePrints/Player/STRUCT_SelectableFirstDiscoverer` (`/Game/MyGame/BluePrints/Player/BP_Player.SelectingFirstDiscoverer` (`self.Player`))))
  (`parent.ReceiveTick` DeltaSeconds)
  (`/Engine/EditorBlueprintResources/StandardMacros.IsValid` _selectingfirstdiscoverer_audience_2
    (:`Is Valid`
      (bind _isfinish (`self.MoveCamera` (`/Game/MyGame/BluePrints/Audience/BP_CameraSplineBaseToAudience.Spline` (`/Game/MyGame/BluePrints/Accident/BP_Accident.CameraSpline` (`/Game/MyGame/BluePrints/Audience/BP_Audience.Accident` _selectingfirstdiscoverer_audience_2))) 5.0 130.0 8000.0))
      (if _isfinish
        (set `/Game/MyGame/BluePrints/Player/BP_Player.Parent` _selectingfirstdiscoverer_audience (`self.Player`))
        (`/Game/MyGame/BluePrints/Player/BP_Player.FinishMoveCamera` (`self.Player`))
        (`/Game/MyGame/BluePrints/Player/BP_Player.ChangeState` _player "/Game/MyGame/BluePrints/Player/BP_PlayerState_Audience.BP_PlayerState_Audience_C" (`/Game/MyGame/BluePrints/Player/BP_Player.State` _player))))
    (:`Is Not Valid`
      (`/Game/MyGame/BluePrints/Player/BP_Player.FinishMoveCamera` (`self.Player`))
      (`/Game/MyGame/BluePrints/Player/BP_Player.ChangeState` _player_2 "/Game/MyGame/BluePrints/Player/BP_PlayerState_AudienceToBase.BP_PlayerState_AudienceToBase_C" (`/Game/MyGame/BluePrints/Player/BP_Player.State` _player_2)))))

(fn `MoveCamera`
  (params (Spline :type "SplineComponent Object Reference") (FovChangeSpeed :type "Float (double-precision)") (MovingFov :type "Float (double-precision)") (MoveSpeed :type "Float (double-precision)"))
  (returns (IsFinish :type Boolean))
  (locals (SplineTemp :type "SplineComponent Object Reference"))
  (bind _defaultfov (`/Game/MyGame/BluePrints/Player/BP_Player.DefaultFOV` (`self.Player`)))
  ;[1 1 1] FOV徐々に切り替え
  (bind _output_get (set `local.SplineTemp` Spline))
  (`CameraComponent.SetFieldOfView` (`/Game/MyGame/BluePrints/Player/BP_Player.MovingCamera` (`self.Player`)) (+ (* (`KismetMathLibrary.FMin` (* (- 1.0 (* (`KismetMathLibrary.Abs` (- (/ (`self.CameraSplineLength`) (`SplineComponent.GetSplineLength` _output_get)) 0.5)) 2.0)) FovChangeSpeed) 1.0) (- MovingFov _defaultfov)) _defaultfov))
  ;[1 1 1] Spline上を移動
  (bind _output_get_2 (set `self.CameraSplineLength` (+ (`self.CameraSplineLength`) (* (`GameplayStatics.GetWorldDeltaSeconds`) MoveSpeed))))
  (if (<= _output_get_2 (`SplineComponent.GetSplineLength` (`local.SplineTemp`)))
    (`self.K2_SetActorLocation` (`self.Player`) (`SplineComponent.GetLocationAtDistanceAlongSpline` (`local.SplineTemp`) _output_get_2 "World") false false)
    ;[1 1 1] カメラ向き
    (`SceneComponent.K2_SetWorldRotation` (`/Game/MyGame/BluePrints/Player/BP_Player.MovingCamera` (`self.Player`)) (`KismetMathLibrary.FindLookAtRotation` (`self.K2_GetActorLocation` (`self.Player`)) (`SplineComponent.GetLocationAtDistanceAlongSpline` (`local.SplineTemp`) (+ (`self.CameraSplineLength`) 100.0) "World")) false false)
    (return false)
    (else
      (set `self.CameraSplineLength` 0.0)
      (return true))))

(fn `UserConstructionScript`
  (`parent.UserConstructionScript`))