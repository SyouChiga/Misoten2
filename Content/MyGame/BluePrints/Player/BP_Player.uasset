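; Player camera actor that jumps between the base and walkers, dispatching emergency workers to accidents the walkers witness.
; At the base it looks freely and possesses whatever a centre-screen line trace hits by attaching to its CameraPoint.
; Inside a walker, a sight collision gathers and highlights nearby walkers, which look input cycles through as the next jump target.
; Dispatch widgets appear on accident-watching walkers; choosing red spawns a firefighter from the fire station.
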(event `self.ReceiveBeginPlay`
  (bind _returnvalue (`|CreateWidget` "/Game/MyGame/BluePrints/Stage01/Widgets/BPW_Dispatch.BPW_Dispatch_C"))
  (bind _output_get (set `self.Dispatch` _returnvalue))
  (`UserWidget.AddToViewport` _output_get 0)
  (`Widget.SetVisibility` (`self.Dispatch`) "Hidden")
  (bind _returnvalue_2 (`|CreateWidget` "/Game/MyGame/BluePrints/Stage01/Widgets/BPW_SelectWorker.BPW_SelectWorker_C"))
  (bind _output_get_2 (set `self.SelectingWorkerUI` _returnvalue_2))
  (`UserWidget.AddToViewport` _output_get_2 0)
  (`Widget.SetVisibility` (`self.SelectingWorkerUI`) "Hidden"))

(event `self.ReceiveTick`
  (params (DeltaSeconds :type "Float (single-precision)"))
  (`|ExecutionSequence`
    (:`then_0`
      (`/Engine/EditorBlueprintResources/StandardMacros.DoOnce` false
        (:`Completed`
          ;[1 1 1] 参照取得
          (bind _outactors (`GameplayStatics.GetAllActorsOfClass` "/Game/MyGame/BluePrints/BP_Base.BP_Base_C"))
          (set `self.Base` (`|GetArrayItem` _outactors))
          (bind _outactors_2 (`GameplayStatics.GetAllActorsOfClass` "/Game/MyGame/BluePrints/Accident/BP_AccidentGenerator.BP_AccidentGenerator_C"))
          (set `self.AccidentGenerator` (`|GetArrayItem` _outactors_2))
          (bind _outactors_3 (`GameplayStatics.GetAllActorsOfClass` "/Game/MyGame/BluePrints/Station/BP_FireStation.BP_FireStation_C"))
          (set `self.FireStation` (`|GetArrayItem` _outactors_3)))))))

(event `InputAxis|LookRight`
  (params (AxisValue :type "Float (single-precision)"))
  (bind _camera (`self.Camera`))
  (bind _returnvalue (`SceneComponent.GetRelativeTransform` _camera))
  ;[1 1 1] 主観視点カメラ
  (switch `/Game/MyGame/BluePrints/Player/ENUM_PlayerCameraState` (`self.CameraState`)
    (:`NewEnumerator0`
      ;;[1 1 1] ベース時制限無し
      (`SceneComponent.K2_AddLocalRotation` (`self.Camera`) (`KismetMathLibrary.MakeRotator` 0.0 0.0 AxisValue) false false)
      ;;[1 1 1] Roll対策
      (`SceneComponent.K2_SetRelativeRotation` _camera (`KismetMathLibrary.MakeRotator` 0.0 (.pitch (.rotation _returnvalue)) (.yaw (.rotation _returnvalue))) false false))
    (:`NewEnumerator1`
      (if (>= (`KismetMathLibrary.Abs` AxisValue) 0.1)
        (`KismetSystemLibrary.Delay` 0.2)
        (if (> (`self.GetInputAxisValue`) 0.0)
          (`self.ChangeSelectingWalker` (+ (`self.SelectingWalkerIndex`) 1) "/Game/MyGame/Materials/M_Yellow.M_Yellow")
          (else
            (`self.ChangeSelectingWalker` (- (`self.SelectingWalkerIndex`) 1) "/Game/MyGame/Materials/M_Yellow.M_Yellow")))))))

(event `InputAction|ChangeCamera`
  (params (Key :type "Key Structure"))
  (bind _camera (`self.Camera`))
  (bind _selectingwalker (`self.SelectingWalker`))
  (bind _returnvalue (`SceneComponent.K2_GetComponentLocation` _camera))
  ;[1 1 1] 画面中心に捉えたモブまたはベースに乗り移る
  (:`Pressed`
    (if (`|EnumEquality` (`self.CameraState`) "NewEnumerator0")
      (bind _outhit (`KismetSystemLibrary.LineTraceSingle` _returnvalue (+ _returnvalue (* (`SceneComponent.GetForwardVector` _camera) (`self.LineTraceLength`))) "TraceTypeQuery1" false (`|MakeArray` (`self.Parent`))))
      (`|ExecutionSequence`
        (:`then_0`
          ;;[1 1 1] モブに乗り移り
          (bind _asbp_walker (cast `/Game/MyGame/BluePrints/Walker/BP_Walker` (`.HitActor` (`GameplayStatics.BreakHitResult` _outhit))))
          (`self.ChangeCameraToWalker` _asbp_walker))
        (:`then_1`
          ;;[1 1 1] ベースに乗り移り
          (bind _asbp_base (cast `/Game/MyGame/BluePrints/BP_Base` (`.HitActor` (`GameplayStatics.BreakHitResult` _outhit))))
          (`self.ChangeCameraToBase` _asbp_base)))
      (else
        (`/Engine/EditorBlueprintResources/StandardMacros.IsValid` _selectingwalker
          (:`Is Valid`
            (`self.ChangeCameraToWalker` _selectingwalker)))))))

(event `InputAxis|LookUp`
  (params (AxisValue :type "Float (single-precision)"))
  (bind _lookuplimit (`self.LookUpLimit`))
  (bind _returnvalue (`SceneComponent.GetRelativeTransform` (`self.Camera`)))
  ;[1 1 1] 主観視点カメラ
  ;;[1 1 1] 上下角度制限
  (if (>= AxisValue 0.0)
    (if (<= (.pitch (.rotation _returnvalue)) _lookuplimit)
      (`SceneComponent.K2_AddLocalRotation` (`self.Camera`) (`KismetMathLibrary.MakeRotator` 0.0 AxisValue) false false :!label _label))
    (elif (>= (.pitch (.rotation _returnvalue)) (* _lookuplimit -1.0))
      (goto _label))))

(event `InputAction|ReturnToBase`
  (params (Key :type "Key Structure"))
  ;[1 1 1] ベースに乗り移り
  (:`Pressed`
    (`self.ChangeCameraToBase` (`self.Base`))))

(event `InputAction|Dispatch`
  (params (Key :type "Key Structure"))
  ;[1 1 1] 出動
  (:`Pressed`
    (switch `/Game/MyGame/BluePrints/Player/ENUM_PlayerCameraState` (`self.CameraState`)
      (:`NewEnumerator1`
        (bind _asbp_walker (cast `/Game/MyGame/BluePrints/Walker/BP_Walker` (`self.Parent`)))
        (switch `/Game/MyGame/BluePrints/Walker/ENUM_WalkerState` (`/Game/MyGame/BluePrints/Walker/BP_Walker.State` _asbp_walker)
          (:`NewEnumerator1`
            (switch `/Game/MyGame/BluePrints/Stage01/Widgets/ENUM_SelectImage` (`/Game/MyGame/BluePrints/Stage01/Widgets/BPW_SelectWorker.GetSelectImg` (`self.SelectingWorkerUI`))
              (:`NewEnumerator0`
                (`/Game/MyGame/BluePrints/Station/BP_Station.SpawnWorker` (`self.FireStation`) "/Game/MyGame/BluePrints/Worker/BP_FireFighter.BP_FireFighter_C" (`/Game/MyGame/BluePrints/Walker/BP_Walker.LookingAccident` _asbp_walker))))))))))

(event `self.OnSightCollision.OnComponentBeginOverlap`
  (params (OverlappedComponent :type "PrimitiveComponent Object Reference") (OtherActor :type "Actor Object Reference") (OtherComp :type "PrimitiveComponent Object Reference") (OtherBodyIndex :type Integer) (bFromSweep :type Boolean) (SweepResult :type "HitResult Structure (by ref)"))
  (if (`|EnumEquality` (`self.CameraState`) "NewEnumerator1")
    (bind _asbp_walker (cast `/Game/MyGame/BluePrints/Walker/BP_Walker` OtherActor))
    (if (not (`/Game/MyGame/BluePrints/Walker/BP_Walker.OnSight` _asbp_walker))
      (set `/Game/MyGame/BluePrints/Walker/BP_Walker.OnSight` true _asbp_walker)
      ;[1 1 1] リストに追加
      (`KismetArrayLibrary.Array_Add` (`self.WalkerArray`) _asbp_walker)
      ;[1 1 1] 選択可能な奴のマテリアル変更
      (`PrimitiveComponent.SetMaterial` (`Character.Mesh` _asbp_walker) 0 (`self.OnSightWalkerMaterial`))
      ;[1 1 1] 配列に一番最初に追加したやつは現在選択中にしてマテリアルを選択中マテリアルに
      (if (== (`KismetArrayLibrary.Array_Length` (`self.WalkerArray`)) 1)
        (set `self.SelectingWalker` _asbp_walker)
        (set `self.SelectingWalkerIndex` 0)
        (`PrimitiveComponent.SetMaterial` (`Character.Mesh` _asbp_walker) 0 (`self.SelectingWalkerMaterial`))))))

(event `self.OnSightCollision.OnComponentEndOverlap`
  (params (OverlappedComponent :type "PrimitiveComponent Object Reference") (OtherActor :type "Actor Object Reference") (OtherComp :type "PrimitiveComponent Object Reference") (OtherBodyIndex :type Integer))
  (bind _asbp_walker (cast `/Game/MyGame/BluePrints/Walker/BP_Walker` OtherActor))
  (if (`/Game/MyGame/BluePrints/Walker/BP_Walker.OnSight` _asbp_walker)
    (set `/Game/MyGame/BluePrints/Walker/BP_Walker.OnSight` false _asbp_walker)
    (`/Game/MyGame/BluePrints/Walker/BP_Walker.MaterialReset` _asbp_walker true)
    ;[1 1 1] 範囲から外れたもぶを配列から削除、インデックスを0に
    (`KismetArrayLibrary.Array_RemoveItem` (`self.WalkerArray`) _asbp_walker)
    (set `self.SelectingWalkerIndex` 0)
    ;[1 1 1] 配列から削除したやつが現在選択中だった場合
    (`|ExecutionSequence`
      (:`then_0`
        (if (== (`self.SelectingWalker`) _asbp_walker)
          (if (> (`KismetArrayLibrary.Array_Length` (`self.WalkerArray`)) 0)
            (`self.ChangeSelectingWalker` 0 "/Game/Mannequin/Character/Materials/M_UE4Man_Body.M_UE4Man_Body")
            (else
              (set `self.SelectingWalker` (`self.NullWalker`)))))))))

(fn `ChangeCameraToBase`
  (params (Base :type "/Game/MyGame/BluePrints/BP_Base Object Reference"))
  (`|ExecutionSequence`
    (:`then_0`
      (set `self.Parent` Base)
      (`self.K2_AttachToComponent` (`/Game/MyGame/BluePrints/BP_Base.CameraPoint` Base) "None" "KeepRelative" "KeepRelative" "KeepRelative")
      (`self.K2_SetActorRelativeLocation` (0.0 0.0 0.0))
      (`SceneComponent.K2_SetRelativeRotation` :`self` (`self.Camera`))
      (set `self.CameraState` "NewEnumerator0")
      (`self.HiddenDispatch`))))

(fn `ChangeCameraToWalker`
  (params (Walker :type "/Game/MyGame/BluePrints/Walker/BP_Walker Object Reference"))
  (`|ExecutionSequence`
    (:`then_0`
      (set `self.Parent` Walker)
      (`self.K2_AttachToComponent` (`/Game/MyGame/BluePrints/Walker/BP_Walker.CameraPoint` Walker) "None" "KeepRelative" "KeepRelative" "KeepWorld")
      (`self.K2_SetActorRelativeLocation` (0.0 0.0 0.0))
      (`SceneComponent.K2_SetRelativeRotation` :`self` (`self.Camera`))
      (set `self.CameraState` "NewEnumerator1"))
    (:`then_1`
      (switch `/Game/MyGame/BluePrints/Walker/ENUM_WalkerState` (`/Game/MyGame/BluePrints/Walker/BP_Walker.State` Walker)
        (:`NewEnumerator0`
          (`self.HiddenDispatch`))
        (:`NewEnumerator1`
          (`self.VisibleDispatch`))))))

(fn `ChangeSelectingWalker`
  (params (IndexWalker :type Integer) (SelectedWalkerMat :type "Material Object Reference"))
  (locals (NewSelectingWalkerIndex :type Integer) (SelectedWalkerMaterial :type "Material Object Reference"))
  (bind _selectingwalker (`self.SelectingWalker`))
  (bind _output_get (set `local.NewSelectingWalkerIndex` IndexWalker))
  (set `local.SelectedWalkerMaterial` SelectedWalkerMat)
  ;[1 1 1] 指定されたIndexでWalkerが存在していれば処理続行
  (`/Engine/EditorBlueprintResources/StandardMacros.IsValid` (`|GetArrayItem` (`self.WalkerArray`) _output_get)
    (:`Is Valid`
      ;[1 1 1] 選択可能のマテリアルに戻す
      (`/Engine/EditorBlueprintResources/StandardMacros.IsValid` _selectingwalker
        (:`Is Valid`
          (`PrimitiveComponent.SetMaterial` (`Character.Mesh` _selectingwalker) 0 (`local.SelectedWalkerMaterial`)))
        (:`Is Not Valid`
          _))
      ;[1 1 1] 新しいやつに更新
      (bind _output_get_2 (set `self.SelectingWalker` (`|GetArrayItem` (`self.WalkerArray`) (`local.NewSelectingWalkerIndex`))))
      (`PrimitiveComponent.SetMaterial` (`Character.Mesh` _output_get_2) 0 (`self.SelectingWalkerMaterial`))
      ;[1 1 1] Indexも一応更新
      (set `self.SelectingWalkerIndex` (`local.NewSelectingWalkerIndex`)))))

(fn `GetControllerAxisX`
  (returns (AxisX :type "Float (double-precision)"))
  (return (`self.GetInputAxisKeyValue`)))

(fn `GetControllerAxisY`
  (returns (AxisY :type "Float (double-precision)"))
  (return (* (`self.GetInputAxisKeyValue`) -1.0)))

(fn `HiddenDispatch`
  (`Widget.SetVisibility` (`self.Dispatch`) "Hidden")
  (`Widget.SetVisibility` (`self.SelectingWorkerUI`) "Hidden")
  (`self.ResetWalkerArray`))

(fn `ResetWalkerArray`
  (for _array_element (`self.WalkerArray`)
    (set `/Game/MyGame/BluePrints/Walker/BP_Walker.OnSight` false _array_element)
    (`/Game/MyGame/BluePrints/Walker/BP_Walker.MaterialReset` _array_element true)
    (`KismetArrayLibrary.Array_RemoveItem` (`self.WalkerArray`) _array_element))
  (set `self.SelectingWalkerIndex` 0)
  (set `self.SelectingWalker` (`self.NullWalker`))
  (return))

(fn `UserConstructionScript`)

(fn `VisibleDispatch`
  (`Widget.SetVisibility` (`self.Dispatch`) "Visible")
  (`Widget.SetVisibility` (`self.SelectingWorkerUI`) "Visible"))