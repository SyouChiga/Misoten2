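; Player state for the base camera view, where the player picks an accident's first discoverer to switch to that audience member's camera.
; Each tick it rebuilds the selectable list from AccidentGenerator and smoothly turns the camera toward the selection, or slowly rotates it when none exists.
; A lost selection falls back to the nearest by dot product, or resets.
; Left/right inputs cycle targets; ChangeCamera transitions to BP_PlayerState_BaseToAudience.
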(event `self.ReceiveTick`
  (params (DeltaSeconds :type "Float (single-precision)"))
  (bind _player (`self.Player`))
  (bind _player_2 (`self.Player`))
  (bind _selectingfirstdiscoverer_audience (break `/Game/MyGame/BluePrints/Player/STRUCT_SelectableFirstDiscoverer` (`/Game/MyGame/BluePrints/Player/BP_Player.SelectingFirstDiscoverer` (`self.Player`))))
  (bind (_selectingfirstdiscoverer_audience_2 _selectingfirstdiscoverer_isvaliable) (break `/Game/MyGame/BluePrints/Player/STRUCT_SelectableFirstDiscoverer` (`/Game/MyGame/BluePrints/Player/BP_Player.SelectingFirstDiscoverer` (`self.Player`))))
  (bind (_returnvalue_location _returnvalue_rotation) (`KismetMathLibrary.BreakTransform` (`SceneComponent.K2_GetComponentToWorld` (`/Game/MyGame/BluePrints/Player/BP_Player.BaseCamera` _player_2))))
  (`|ExecutionSequence`
    (:`then_0`
      ;[1 1 1] 選択可能なFirstDiscoverer検出
      (`/Game/MyGame/BluePrints/Player/BP_Player.ClearSelectableFirstDiscoverers` (`self.Player`))
      (for _array_element (`/Game/MyGame/BluePrints/Accident/BP_AccidentGenerator.Accidents` (`/Game/MyGame/BluePrints/Player/BP_Player.AccidentGenerator` (`self.Player`)))
        (bind _firstdiscoverer (`/Game/MyGame/BluePrints/Accident/BP_Accident.FirstDiscoverer` _array_element))
        (`/Engine/EditorBlueprintResources/StandardMacros.IsValid` _firstdiscoverer
          (:`Is Valid`
            (`/Game/MyGame/BluePrints/Player/BP_Player.AddSelectableFirstDiscoverer` (`self.Player`) _firstdiscoverer)))))
    (:`then_1`
      ;[1 1 1] 選択中のFirstDiscovererの有無
      (if _selectingfirstdiscoverer_isvaliable
        (`|ExecutionSequence`
          (:`then_0`
            ;[1 1 1] カメラ回転
            (`SceneComponent.K2_SetWorldRotation` (`/Game/MyGame/BluePrints/Player/BP_Player.BaseCamera` (`self.Player`)) (`KismetMathLibrary.RInterpTo` _returnvalue_rotation (`KismetMathLibrary.FindLookAtRotation` (`self.K2_GetActorLocation` _player_2) (`self.K2_GetActorLocation` _selectingfirstdiscoverer_audience)) (`GameplayStatics.GetWorldDeltaSeconds`) 5.0) false false))
          (:`then_1`
            ;[1 1 1] 選択中のFirstDiscovererが存在するか判定
            (bind _isexist (`/Game/MyGame/BluePrints/Player/BP_Player.IsExistSelectingFirstDiscovererInSelectableFirstDiscoverers` (`self.Player`)))
            (if (not _isexist)
              ;[1 1 1] 他のFirstDiscovererが存在する場合、内積値の最も近いFirstDiscovererを選択する　無い場合は無効化してカメラをリセット
              (if (> (`KismetArrayLibrary.Array_Length` (`/Game/MyGame/BluePrints/Player/BP_Player.SelectableFirstDiscoverers` (`self.Player`))) 0)
                (`/Game/MyGame/BluePrints/Player/BP_Player.SelectNearInnerFirstDiscoverer` _player)
                (else
                  (`/Game/MyGame/BluePrints/Player/BP_Player.SetSelectingFirstDiscoverer` :`self` _player)
                  (`SceneComponent.K2_SetRelativeRotation` :`self` (`/Game/MyGame/BluePrints/Player/BP_Player.BaseCamera` (`self.Player`))))))))
        (else
          ;[1 1 1] カメラデフォルト位置
          (`SceneComponent.K2_AddRelativeRotation` (`/Game/MyGame/BluePrints/Player/BP_Player.BaseCamera` (`self.Player`)) (struct :`Yaw` 0.1) false false)
          ;[1 1 1] 選択可能なFirstDiscovererがいる場合選択する
          (if (> (`KismetArrayLibrary.Array_Length` (`/Game/MyGame/BluePrints/Player/BP_Player.SelectableFirstDiscoverers` (`self.Player`))) 0)
            (`/Game/MyGame/BluePrints/Player/BP_Player.SetSelectingFirstDiscoverer` (`self.Player`) (`|GetArrayItem` (`/Game/MyGame/BluePrints/Player/BP_Player.SelectableFirstDiscoverers` (`self.Player`))))))))))

(event `self.ChangeCamera`
  (bind (_selectingfirstdiscoverer_audience _selectingfirstdiscoverer_isvaliable) (break `/Game/MyGame/BluePrints/Player/STRUCT_SelectableFirstDiscoverer` (`/Game/MyGame/BluePrints/Player/BP_Player.SelectingFirstDiscoverer` (`self.Player`))))
  (if _selectingfirstdiscoverer_isvaliable
    (`/Game/MyGame/BluePrints/Player/BP_Player.StartMoveCamera` (`self.Player`))
    (`/Game/MyGame/BluePrints/Player/BP_Player.SwitchToAudienceCamera` (`self.Player`))
    (`/Game/MyGame/BluePrints/Player/BP_Player.ChangeState` (`self.Player`) "/Game/MyGame/BluePrints/Player/BP_PlayerState_BaseToAudience.BP_PlayerState_BaseToAudience_C" self)))

(event `self.SelectRight`
  (if (> (`KismetArrayLibrary.Array_Length` (`/Game/MyGame/BluePrints/Player/BP_Player.SelectableFirstDiscoverers` (`self.Player`))) 1)
    (`/Game/MyGame/BluePrints/Player/BP_Player.SelectRightFirstDiscoverer` (`self.Player`))))

(event `self.SelectLeft`
  (if (> (`KismetArrayLibrary.Array_Length` (`/Game/MyGame/BluePrints/Player/BP_Player.SelectableFirstDiscoverers` (`self.Player`))) 1)
    (`/Game/MyGame/BluePrints/Player/BP_Player.SelectLeftFirstDiscoverer` (`self.Player`))))

(fn `UserConstructionScript`
  (`parent.UserConstructionScript`))