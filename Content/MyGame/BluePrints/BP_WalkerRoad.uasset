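; BP_WalkerRoad is a spline-driven road actor that lays repeated mesh pieces along an editable path.
; The construction script adds Num instances to an InstancedStaticMesh at evenly spaced distances along the spline, each aligned to the spline's local position and rotation.
; Length, Width and Height set every instance's scale, and the event graph holds no runtime logic.
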(fn `UserConstructionScript`
  (for _index (range (`self.Num`))
    (bind _returnvalue (* (/ (`KismetMathLibrary.Conv_IntToDouble` _index) (`KismetMathLibrary.Conv_IntToDouble` (`self.Num`))) (`SplineComponent.GetSplineLength` (`self.Spline`))))
    (`InstancedStaticMeshComponent.AddInstance` (`self.InstancedStaticMesh`) (`KismetMathLibrary.MakeTransform` (`SplineComponent.GetLocationAtDistanceAlongSpline` (`self.Spline`) _returnvalue "Local") (`SplineComponent.GetRotationAtDistanceAlongSpline` (`self.Spline`) _returnvalue "Local") (`KismetMathLibrary.MakeVector` (`self.Length`) (`self.Width`) (`self.Height`))))))