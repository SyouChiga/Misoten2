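; BPGM_Stage01 is the Stage 01 Blueprint, apparently its Game Mode, that sets up the player and screen UI when play begins.
; PlayerSpawn spawns BP_Player, attaches it to the CameraPoint of the first BP_Base found in the level, and has player controller 0 possess it.
; BeginPlay then adds the BPW_Center widget to the viewport, and an Escape input event quits the game.
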(event `self.ReceiveBeginPlay`
  (`self.PlayerSpawn`)
  (bind _returnvalue (`|CreateWidget` "/Game/MyGame/BluePrints/Stage01/Widgets/BPW_Center.BPW_Center_C"))
  (bind _output_get (set `self.CenterWidget` _returnvalue))
  (`UserWidget.AddToViewport` _output_get 0))

(event `self.ReceiveTick`
  (params (DeltaSeconds :type "Float (single-precision)")))

(event `InputAction|Escape`
  (params (Key :type "Key Structure"))
  (:`Pressed`
    (`KismetSystemLibrary.QuitGame` null "Quit")))

(fn `PlayerSpawn`
  (bind _outactors (`GameplayStatics.GetAllActorsOfClass` "/Game/MyGame/BluePrints/BP_Base.BP_Base_C"))
  (bind _output (`|GetArrayItem` _outactors))
  (bind _returnvalue (`|SpawnActorFromClass` "/Game/MyGame/BluePrints/BP_Player.BP_Player_C" (`KismetMathLibrary.MakeTransform` (0.0 0.0 0.0)) "AlwaysSpawn" "OverrideRootScale" null _output null))
  (`self.K2_AttachToComponent` _returnvalue (`/Game/MyGame/BluePrints/BP_Base.CameraPoint` _output) "None" "KeepRelative" "KeepRelative" "KeepRelative" true)
  (`Controller.Possess` (`GameplayStatics.GetPlayerController` 0) _returnvalue))

(fn `UserConstructionScript`)