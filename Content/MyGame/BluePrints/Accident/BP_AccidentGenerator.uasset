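; Actor that periodically rolls to spawn fire accidents at free BP_AccidentLocation actors in the level, with odds depending on whether any accident is active.
; Each spawn picks a random free location, passes it the worker spawn point and camera spline, and creates audience actors flagged for dispatch ability and first discoverer.
; DestroyAccident unregisters the accident; only if the player is in Audience state does it reset the camera and destroy the audiences and accident.
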(event `self.ReceiveTick`
  (params (DeltaSeconds :type "Float (single-precision)"))
  (`|ExecutionSequence`
    (:`then_0`
      (`/Engine/EditorBlueprintResources/StandardMacros.DoOnce` false
        (:`Completed`
          (bind _outactors (`GameplayStatics.GetAllActorsOfClass` "/Game/MyGame/BluePrints/Accident/BP_AccidentLocation.BP_AccidentLocation_C"))
          (set `self.AccidentLocations` _outactors)
          (bind _asbp_player (cast `/Game/MyGame/BluePrints/Player/BP_Player` (`GameplayStatics.GetPlayerPawn` 0)))
          (set `self.Player` _asbp_player))))
    (:`then_1`
      ;[1 1 1] 一定周期で抽選を行いアクシデント生成
      (bind _output_get (set `self.Delay` (+ (`GameplayStatics.GetWorldDeltaSeconds`) (`self.Delay`))))
      (if (< (`self.DelayValue`) _output_get)
        (set `self.Delay` 0.0)
        (if (== (`KismetArrayLibrary.Array_Length` (`self.Accidents`)) 0)
          ;;[1 1 1] 1つもアクシデントが無い場合
          (if (< (`KismetMathLibrary.RandomFloatInRange` 0.0 100.0) (`self.NoAccidentProbability`))
            (`self.SpawnAccidentRandom` "/Game/MyGame/BluePrints/Accident/BP_FireAccident.BP_FireAccident_C" :!label _label))
          (else
            ;;[1 1 1] 1つ以上アクシデントがある場合
            (if (< (`KismetMathLibrary.RandomFloatInRange` 0.0 100.0) (`self.OneAccidentProbability`))
              (goto _label))))))))

(fn `DestroyAccident`
  (params (Accident :type "/Game/MyGame/BluePrints/Accident/BP_Accident Object Reference (by ref)"))
  (locals (AccidentTemp :type "/Game/MyGame/BluePrints/Accident/BP_Accident Object Reference"))
  (bind _output_get (set `local.AccidentTemp` Accident))
  (`KismetArrayLibrary.Array_RemoveItem` (`self.Accidents`) _output_get)
  ;[1 1 1] アクシデントが消えた時点でAudienceにいた場合Baseに戻る
  (cast `/Game/MyGame/BluePrints/Player/BP_PlayerState_Audience` (`/Game/MyGame/BluePrints/Player/BP_Player.State` (`self.Player`)))
  (`/Game/MyGame/BluePrints/Player/BP_Player.ChangeCameraToBase` (`self.Player`))
  ;[1 1 1] Audienceも破棄
  (for _array_element (`/Game/MyGame/BluePrints/Accident/BP_Accident.Audiences` (`local.AccidentTemp`))
    (`self.K2_DestroyActor` _array_element))
  (`self.K2_DestroyActor` (`local.AccidentTemp`)))

(fn `IsCanDispatchAudienceLocation`
  (params (AudienceLocation :type "/Game/MyGame/BluePrints/Audience/BP_AudienceLocation Object Reference") (AccidentLocation :type "/Game/MyGame/BluePrints/Accident/BP_AccidentLocation Object Reference"))
  (returns (IsCanDispatch :type Boolean))
  (for _array_element (`/Game/MyGame/BluePrints/Accident/BP_AccidentLocation.CanDispatchAudienceLocations` AccidentLocation)
    (if (== _array_element AudienceLocation)
      (return true)))
  (return false))

(fn `SpawnAccident`
  (params (AccidentClass :type "/Game/MyGame/BluePrints/Accident/BP_Accident Class Reference") (Location :type "Vector Structure") (WorkerSpawnPoint :type "/Game/MyGame/BluePrints/Accident/BP_WorkerSpawnPoint Object Reference") (CameraSpline :type "/Game/MyGame/BluePrints/Audience/BP_CameraSplineBaseToAudience Object Reference"))
  (returns (Accident :type "/Game/MyGame/BluePrints/Accident/BP_Accident Object Reference"))
  (bind _returnvalue (`|SpawnActorFromClass` AccidentClass (`KismetMathLibrary.MakeTransform` Location) "AlwaysSpawn" "OverrideRootScale" null self WorkerSpawnPoint CameraSpline null))
  (`KismetArrayLibrary.Array_Add` (`self.Accidents`) _returnvalue)
  (return _returnvalue))

(fn `SpawnAccidentRandom`
  (params (AccidentClass :type "/Game/MyGame/BluePrints/Accident/BP_Accident Class Reference"))
  (locals (ProposedLocations :type "Array of /Game/MyGame/BluePrints/Accident/BP_AccidentLocation Object Reference") (SelectedProposedLocation :type "/Game/MyGame/BluePrints/Accident/BP_AccidentLocation Object Reference") (SpawnAccidentClass :type "/Game/MyGame/BluePrints/Accident/BP_Accident Class Reference"))
  (bind _selectedproposedlocation (`local.SelectedProposedLocation`))
  (set `local.SpawnAccidentClass` AccidentClass)
  ;[1 1 1] Spawn可能な候補検索
  (for _array_element (`self.AccidentLocations`)
    (`/Engine/EditorBlueprintResources/StandardMacros.IsValid` (`/Game/MyGame/BluePrints/Accident/BP_AccidentLocation.Accident` _array_element)
      (:`Is Not Valid`
        (`KismetArrayLibrary.Array_Add` (`local.ProposedLocations`) _array_element))))
  ;[1 1 1] Spawn可能な候補の有無
  (if (> (`KismetArrayLibrary.Array_Length` (`local.ProposedLocations`)) 0)
    ;[1 1 1] Spawn可能な候補からランダムで選択
    (set `local.SelectedProposedLocation` (`|GetArrayItem` (`local.ProposedLocations`) (`KismetMathLibrary.RandomIntegerInRange` 0 (- (`KismetArrayLibrary.Array_Length` (`local.ProposedLocations`)) 1))))
    ;[1 1 1] AccidentをSpawn　AccidentにWorkerの生成位置とカメラ用Splineの参照変数セット
    (bind _accident (`self.SpawnAccident` (`local.SpawnAccidentClass`) (`self.K2_GetActorLocation` _selectedproposedlocation) (`/Game/MyGame/BluePrints/Accident/BP_AccidentLocation.WorkerSpawnPoint` _selectedproposedlocation) (`/Game/MyGame/BluePrints/Accident/BP_AccidentLocation.CameraSpline` _selectedproposedlocation)))
    ;[1 1 1] AccidentLocationにAccidentの参照変数セット
    (set `/Game/MyGame/BluePrints/Accident/BP_AccidentLocation.Accident` _accident (`local.SelectedProposedLocation`))
    ;[1 1 1] Audience生成　Accidentの参照変数と出動要請ができるかどうかのフラグをセット
    (for _array_element_2 (`/Game/MyGame/BluePrints/Accident/BP_AccidentLocation.AudienceLocations` (`local.SelectedProposedLocation`))
      (bind _returnvalue (`|SpawnActorFromClass` "/Game/MyGame/BluePrints/Audience/BP_Audience.BP_Audience_C" (`KismetMathLibrary.MakeTransform` (`self.K2_GetActorLocation` _array_element_2) (`self.K2_GetActorRotation` _array_element_2)) "AlwaysSpawn" "OverrideRootScale" null _accident (`self.IsCanDispatchAudienceLocation` _array_element_2 (`local.SelectedProposedLocation`)) null))
      (`KismetArrayLibrary.Array_Add` (`/Game/MyGame/BluePrints/Accident/BP_Accident.Audiences` _accident) _returnvalue)
      ;;[1 1 1] 第一発見者かどうか
      (if (== _array_element_2 (`/Game/MyGame/BluePrints/Accident/BP_AccidentLocation.FirstDiscovererAudienceLocation` (`local.SelectedProposedLocation`)))
        (set `/Game/MyGame/BluePrints/Accident/BP_Accident.FirstDiscoverer` _returnvalue _accident)))))

(fn `UserConstructionScript`)