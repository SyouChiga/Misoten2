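; BP_FireAccident01 is a fire accident that workers resolve, with firefighters working on it most effectively.
; Its Resolving event casts the Worker to BP_FireFighter and forwards the full WorkSpeed on success, or half of it for any other worker.
; BeginPlay, overlap and Tick are disabled stubs, and the construction script only calls its parent.
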(event `self.Resolving`
  (params (WorkSpeed :type "Float (single-precision)") (Worker :type "/Game/MyGame/BluePrints/Worker/BP_Worker Object Reference"))
  (cast `/Game/MyGame/BluePrints/Worker/FireFighter/BP_FireFighter` Worker
    (:`then`
      (`self.Resolving` WorkSpeed))
    (:`CastFailed`
      (`self.Resolving` (/ WorkSpeed 2.0)))))

(fn `UserConstructionScript`
  (`parent.UserConstructionScript`))