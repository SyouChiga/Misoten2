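; Accident actor that passing BP_Walkers notice and that can be resolved through work.
; Overlapping walkers in the Walking state look at it; one becomes first discoverer, the farthest at spawn or else the first to enter.
; Resolving adds work over time, and Tick has AccidentGenerator destroy the accident once resolved.
; A time-limit check also destroys it, lowering GameState relief, though ProgressTime is never accumulated between ticks.
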(event `self.ReceiveBeginPlay`
  (bind _returnvalue (`self.K2_GetActorLocation`))
  (bind _firstdiscoverer (`self.FirstDiscoverer`))
  (bind _overlappingactors (`PrimitiveComponent.GetOverlappingActors` (`self.WalkerCollision`) "/Game/MyGame/BluePrints/Walker/BP_Walker.BP_Walker_C"))
  ;[1 1 1] 生成時第一発見者検出
  (`|ExecutionSequence`
    (:`then_0`
      (if (> (`KismetArrayLibrary.Array_Length` _overlappingactors) 0)
        (for _array_element _overlappingactors
          (bind _asbp_walker (cast `/Game/MyGame/BluePrints/Walker/BP_Walker` _array_element))
          (switch `/Game/MyGame/BluePrints/Walker/ENUM_WalkerState` (`/Game/MyGame/BluePrints/Walker/BP_Walker.State` _asbp_walker)
            (:`NewEnumerator0`
              (`/Game/MyGame/BluePrints/Walker/BP_Walker.LookAccident` _asbp_walker self)
              (`/Engine/EditorBlueprintResources/StandardMacros.IsValid` (`self.FirstDiscoverer`)
                (:`Is Valid`
                  (if (>= (`KismetMathLibrary.VSizeSquared` (- (`self.K2_GetActorLocation` _asbp_walker) _returnvalue)) (`KismetMathLibrary.VSizeSquared` (- _returnvalue (`self.K2_GetActorLocation` (`self.FirstDiscoverer`)))))
                    (set `self.FirstDiscoverer` _asbp_walker :!label _label)))
                (:`Is Not Valid`
                  (goto _label))))))
        (`/Engine/EditorBlueprintResources/StandardMacros.IsValid` _firstdiscoverer
          (:`Is Valid`
            (`/Game/MyGame/BluePrints/Walker/BP_Walker.BecomeFirstDiscoverer` _firstdiscoverer)))))
    (:`then_1`
      (bind _asbpgs_stage_01 (cast `/Game/MyGame/BluePrints/Stage01/BPGS_Stage01` (`GameplayStatics.GetGameState`)))
      (set `self.GameState` _asbpgs_stage_01))))

(event `self.ReceiveTick`
  (params (DeltaSeconds :type "Float (single-precision)"))
  (`|ExecutionSequence`
    (:`then_0`
      ;[1 1 1] Accident解決チェック
      (bind _isfinish (`self.CheckIsFinish`))
      (if _isfinish
        (`/Game/MyGame/BluePrints/Accident/BP_AccidentGenerator.DestroyAccident` (`self.AccidentGenerator`) self)))
    (:`then_1`
      ;[1 1 1] 経過時間計測　Limit到達でDestroy
      (if (>= (+ (`self.ProgressTime`) (`GameplayStatics.GetWorldDeltaSeconds`)) (`self.ProgressTimeLimit`))
        (`/Game/MyGame/BluePrints/Stage01/BPGS_Stage01.DecReliefValue` (`self.GameState`) 0.1)
        (set `self.ProgressTime` (`self.ProgressTimeLimit`))
        (`/Game/MyGame/BluePrints/Accident/BP_AccidentGenerator.DestroyAccident` (`self.AccidentGenerator`) self)))))

(event `self.WalkerCollision.OnComponentBeginOverlap`
  (params (OverlappedComponent :type "PrimitiveComponent Object Reference") (OtherActor :type "Actor Object Reference") (OtherComp :type "PrimitiveComponent Object Reference") (OtherBodyIndex :type Integer) (bFromSweep :type Boolean) (SweepResult :type "HitResult Structure (by ref)"))
  ;[1 1 1] 第一発見者検出
  (bind _asbp_walker (cast `/Game/MyGame/BluePrints/Walker/BP_Walker` OtherActor))
  (switch `/Game/MyGame/BluePrints/Walker/ENUM_WalkerState` (`/Game/MyGame/BluePrints/Walker/BP_Walker.State` _asbp_walker)
    (:`NewEnumerator0`
      (`/Game/MyGame/BluePrints/Walker/BP_Walker.LookAccident` _asbp_walker self)
      (`/Engine/EditorBlueprintResources/StandardMacros.IsValid` (`self.FirstDiscoverer`)
        (:`Is Not Valid`
          (bind _output_get (set `self.FirstDiscoverer` _asbp_walker))
          (`/Game/MyGame/BluePrints/Walker/BP_Walker.BecomeFirstDiscoverer` _output_get))))))

(fn `CheckIsFinish`
  (returns (IsFinish :type Boolean))
  (return (>= (`self.Resolution`) (`self.ResolutionValue`))))

(fn `Resolving`
  (params (WorkSpeed :type "Float (double-precision)"))
  (set `self.Resolution` (+ (* WorkSpeed (`GameplayStatics.GetWorldDeltaSeconds`)) (`self.Resolution`)))
  (return))

(fn `UserConstructionScript`)