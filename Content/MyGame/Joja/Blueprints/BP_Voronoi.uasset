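; BP_Voronoi is a short-lived actor that drifts upward and grows until it is destroyed after a three-second lifespan.
; BeginPlay picks a mostly vertical direction with a small random horizontal offset.
; Each Tick moves the actor along that direction by Rizespeed without sweeping and adds a fixed increment to its scale.
; Neither step uses delta time, so rise and growth rates depend on frame rate.
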(event `self.ReceiveBeginPlay`
  (set `self.Vec` (`KismetMathLibrary.MakeVector` (`KismetMathLibrary.RandomFloatInRange` -0.3 0.3) (`KismetMathLibrary.RandomFloatInRange` -0.3 0.3) 1.0))
  (`self.SetLifeSpan` 3.0))

(event `self.ReceiveTick`
  (params (DeltaSeconds :type "Float (single-precision)"))
  (`self.K2_SetActorLocation` (+ (* (`self.Vec`) (`self.rizespeed`)) (`self.K2_GetActorLocation`)))
  (`self.SetActorScale3D` (+ (`self.GetActorScale3D`) (0.1 0.1 0.1))))

(fn `UserConstructionScript`)