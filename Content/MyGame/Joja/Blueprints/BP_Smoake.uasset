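; BP_Smoake is a smoke puff actor that drifts upward and expands until it expires after a short lifespan.
; BeginPlay picks an upward vector with random horizontal spread and sets the lifespan.
; Tick moves the actor along that vector by RizeSpeed without sweeping and grows its scale by a fixed step, both per frame with no delta-time scaling.
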(event `self.ReceiveBeginPlay`
  ;[1 1 1] ランダムで拡散する上方向ベクトル
  (set `self.Vec` (`KismetMathLibrary.MakeVector` (`KismetMathLibrary.RandomFloatInRange` -0.3 0.3) (`KismetMathLibrary.RandomFloatInRange` -0.3 0.3) 1.0))
  ;[1 1 1] 煙の寿命
  (`self.SetLifeSpan` 3.0))

(event `self.ReceiveTick`
  (params (DeltaSeconds :type "Float (single-precision)"))
  ;[1 1 1] 上昇させる
  (`self.K2_SetActorLocation` (+ (* (`self.Vec`) (`self.RizeSpeed`)) (`self.K2_GetActorLocation`)))
  ;[1 1 1] 上昇毎に肥大化
  (`self.SetActorScale3D` (+ (`self.GetActorScale3D`) (0.1 0.1 0.1))))

(fn `UserConstructionScript`)